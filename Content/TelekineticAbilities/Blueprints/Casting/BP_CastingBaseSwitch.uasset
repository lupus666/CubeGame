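; BP_CastingBaseSwitch is a casting Blueprint that toggles a telekinetic ability on and off with the Shoot input.
; On each Shoot release it destroys the active Ability actor, or spawns AbilityClass at its own location with the Character passed in when none exists.
; The spawned actor is stored in Ability and is also destroyed when the caster itself is destroyed.
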(event EventDestroyed
  (bind _ability (Variables|Default|GetAbility))
  (Utilities|IsValid _ability
    (:Is%20Valid
      (Actor|DestroyActor _ability))))

(event Input|ActionEvents|InputActionShoot
  (params (Key :type Key%20Structure :default "None"))
  (:Released
    (Utilities|IsValid (Variables|Default|GetAbility)
      (:Is%20Valid
        (Actor|DestroyActor (Variables|Default|GetAbility)))
      (:Is%20Not%20Valid
        (bind _returnvalue (Game|SpawnActorfromClass (Variables|Settings-Ability|GetAbilityClass) (Math|Conversions|ToTransform(Vector) (Transformation|GetActorLocation)) "Undefined" "SelectDefaultAtRuntime" 0 (Variables|Default|GetCharacter) 0))
        (Variables|Default|SetAbility _returnvalue)))))

(fn ConstructionScript
  (|CallParentFunction))