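; BP_CastingBaseHold is a telekinetic casting Blueprint for hold-style abilities, which exist only while the Shoot input is held.
; Pressing Shoot spawns an AbilityClass actor at the caster actor's location, passes it the Character and stores it as Ability.
; Releasing Shoot, or destroying the casting actor, destroys that ability actor if it is still valid.
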(event EventDestroyed
  (bind _ability (Variables|Default|GetAbility))
  (Utilities|IsValid _ability
    (:Is%20Valid
      (Actor|DestroyActor _ability))))

(event Input|ActionEvents|InputActionShoot
  (params (Key :type Key%20Structure :default "None"))
  (:Pressed
    (bind _returnvalue (Game|SpawnActorfromClass (Variables|Settings-Ability|GetAbilityClass) (Math|Conversions|ToTransform(Vector) (Transformation|GetActorLocation)) "Undefined" 0 (Variables|Default|GetCharacter) 0))
    (Variables|Default|SetAbility _returnvalue))
  (:Released
    (Utilities|IsValid (Variables|Default|GetAbility)
      (:Is%20Valid
        (Actor|DestroyActor (Variables|Default|GetAbility))))))

(fn ConstructionScript
  (|CallParentFunction))