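; Casting Blueprint that toggles a continuous telekinetic grab ability when the Shoot input is released.
; The first toggle spawns a BP_AbilityGrabContinous at its own location, passing in the Character, and keeps a reference to it.
; Later toggles clear the ability's target if it has one, or ask it to find one otherwise.
; Destroying the caster also destroys the spawned ability.
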(event Custom|Toggle
  (Utilities|IsValid (Variables|Default|GetAbility)
    (:Is%20Valid
      (Utilities|IsValid (Variables|/Game/TelekineticAbilities/Blueprints/Abilities/BP_AbilityGrabContinous.BP_AbilityGrabContinous_C|GetTarget (Variables|Default|GetAbility))
        (:Is%20Valid
          (Default|ClearTarget (Variables|Default|GetAbility)))
        (:Is%20Not%20Valid
          (Default|FindTarget (Variables|Default|GetAbility)))))
    (:Is%20Not%20Valid
      (bind _returnvalue (Game|SpawnActorfromClass "/Game/TelekineticAbilities/Blueprints/Abilities/BP_AbilityGrabContinous.BP_AbilityGrabContinous_C" (Math|Conversions|ToTransform(Vector) (Transformation|GetActorLocation)) "Undefined" 0 (Variables|Default|GetCharacter) 0))
      (Variables|Default|SetAbility _returnvalue))))

(event EventDestroyed
  (bind _ability (Variables|Default|GetAbility))
  (Utilities|IsValid _ability
    (:Is%20Valid
      (Actor|DestroyActor _ability))))

(event Input|ActionEvents|InputActionShoot
  (params (Key :type Key%20Structure))
  (:Released
    (CallFunction|Toggle)))

(fn ConstructionScript
  (|CallParentFunction))