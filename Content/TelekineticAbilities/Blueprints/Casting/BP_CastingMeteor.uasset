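; BP_CastingMeteor is the casting actor that turns player input into commands for the telekinetic meteor ability.
; On BeginPlay it runs the parent logic, spawns a BP_AbilityMeteor at its own location with the Character passed in, and stores it.
; Target press and release start and stop targeting, while releasing Shoot fires the meteor.
; When destroyed, it also destroys the spawned ability if still valid.
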(event EventBeginPlay
  (|CallParentFunction)
  (bind _returnvalue (Game|SpawnActorfromClass "/Game/TelekineticAbilities/Blueprints/Abilities/BP_AbilityMeteor.BP_AbilityMeteor_C" (Math|Conversions|ToTransform(Vector) (Transformation|GetActorLocation)) "Undefined" 0 (Variables|Default|GetCharacter) 0))
  (Variables|Default|SetAbility _returnvalue))

(event EventDestroyed
  (bind _ability (Variables|Default|GetAbility))
  (Utilities|IsValid _ability
    (:Is%20Valid
      (Actor|DestroyActor _ability))))

(event Input|ActionEvents|InputActionTarget
  (params (Key :type Key%20Structure :default "None"))
  (bind _ability (Variables|Default|GetAbility))
  (:Pressed
    (Default|StartTargeting _ability))
  (:Released
    (Default|StopTargeting _ability)))

(event Input|ActionEvents|InputActionShoot
  (params (Key :type Key%20Structure :default "None"))
  (:Released
    (Default|ShootMeteor (Variables|Default|GetAbility))))

(fn ConstructionScript
  (|CallParentFunction))