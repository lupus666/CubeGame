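; Chargeable casting base Blueprint for telekinetic abilities that spawns an ability actor when fired.
; Shoot spawns the AbilityClass actor at the world origin, passing the current Charge and Character, and stores it as Ability.
; When the casting object is destroyed, it also destroys the stored Ability if still valid.
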(event EventDestroyed
  (bind _ability (Variables|Default|GetAbility))
  (Utilities|IsValid _ability
    (:Is%20Valid
      (Actor|DestroyActor _ability))))

(event EventShoot
  (bind _returnvalue (Game|SpawnActorfromClass (Variables|Settings-Ability|GetAbilityClass) (Math|Transform|MakeTransform "0, 0, 0") "Undefined" 0 (Variables|Default|GetCharge) (Variables|Default|GetCharacter) 0))
  (Variables|Default|SetAbility _returnvalue))

(fn ConstructionScript
  (|CallParentFunction))