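; BP_CastingMultiGrabContinous is a casting Blueprint that turns player input into control of a continuous multi-grab telekinetic ability.
; Pressing Shoot spawns BP_AbilityMultiGrabContinous at its own location and passes it the Character, or destroys the ability if one already exists.
; Releasing Shoot stops the ability's targeting, while releasing Target or destroying the caster destroys the ability.
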(event EventDestroyed
  (bind _ability (Variables|Default|GetAbility))
  (Utilities|IsValid _ability
    (:Is%20Valid
      (Actor|DestroyActor _ability))))

(event Input|ActionEvents|InputActionShoot
  (params (Key :type Key%20Structure))
  (:Pressed
    (Utilities|IsValid (Variables|Default|GetAbility)
      (:Is%20Valid
        (Actor|DestroyActor (Variables|Default|GetAbility)))
      (:Is%20Not%20Valid
        (bind _returnvalue (Game|SpawnActorfromClass "/Game/TelekineticAbilities/Blueprints/Abilities/BP_AbilityMultiGrabContinous.BP_AbilityMultiGrabContinous_C" (Math|Conversions|ToTransform(Vector) (Transformation|GetActorLocation)) "Undefined" 0 (Variables|Default|GetCharacter) 0))
        (Variables|Default|SetAbility _returnvalue))))
  (:Released
    (Utilities|IsValid (Variables|Default|GetAbility)
      (:Is%20Valid
        (Default|StopTargeting (Variables|Default|GetAbility))))))

(event Input|ActionEvents|InputActionTarget
  (params (Key :type Key%20Structure))
  (bind _ability (Variables|Default|GetAbility))
  (:Released
    (Utilities|IsValid _ability
      (:Is%20Valid
        (Actor|DestroyActor _ability)))))

(fn ConstructionScript
  (|CallParentFunction))