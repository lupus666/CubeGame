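; BP_CastingBaseChargable is a base Blueprint for chargeable casting in the telekinetic abilities set.
; Pressing the Shoot input stores the game time in Charge, and releasing it converts the hold duration into a fraction of ChargeTime, capped at one.
; Release then calls the Shoot event, which is empty here, so the actual cast behavior is not defined in this Blueprint.
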(event Custom|Shoot)

(event Input|ActionEvents|InputActionShoot
  (params (Key :type Key%20Structure :default "None"))
  (:Pressed
    (Variables|Default|SetCharge (Utilities|Time|GetGameTimeinSeconds)))
  (:Released
    (Variables|Default|SetCharge (Math|Float|Min(Float) (/ (- (Utilities|Time|GetGameTimeinSeconds) (Variables|Default|GetCharge)) (Variables|Settings-Charge|GetChargeTime)) 1.0))
    (CallFunction|Shoot)))

(fn ConstructionScript
  (|CallParentFunction))