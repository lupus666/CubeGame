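; BP_CastingShooter is a casting Blueprint for a telekinetic ability that targets and shoots through a helper actor.
; On BeginPlay it spawns a BP_AbilityShooter at the Character's location, passing in the Character, and stores it as Shooter.
; Releasing the Target input calls FindTarget on the Shooter, and pressing Shoot calls ShootTarget.
; When destroyed, it also destroys the Shooter if still valid.
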(event EventDestroyed
  (bind _shooter (Variables|Default|GetShooter))
  (Utilities|IsValid _shooter
    (:Is%20Valid
      (Actor|DestroyActor _shooter))))

(event EventBeginPlay
  (bind _character (Variables|Default|GetCharacter))
  (|CallParentFunction)
  (bind _returnvalue (Game|SpawnActorfromClass "/Game/TelekineticAbilities/Blueprints/Abilities/BP_AbilityShooter.BP_AbilityShooter_C" (Math|Conversions|ToTransform(Vector) (Transformation|GetActorLocation _character)) "Undefined" 0 _character 0))
  (Variables|Default|SetShooter _returnvalue))

(event Input|ActionEvents|InputActionTarget
  (params (Key :type Key%20Structure :default "None"))
  (:Released
    (Default|FindTarget (Variables|Default|GetShooter))))

(event Input|ActionEvents|InputActionShoot
  (params (Key :type Key%20Structure :default "None"))
  (:Pressed
    (Default|ShootTarget (Variables|Default|GetShooter))))

(fn ConstructionScript
  (|CallParentFunction))