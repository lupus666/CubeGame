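; Telekinetic anti-gravity ability actor that applies a vertical force to targets inside a spherical area around the caster.
; On BeginPlay it moves to the caster, sizes the sphere from Radius and shows it only in debug, then optionally follows the caster.
; Sphere overlaps maintain a list of telekinetic targets, excluding the caster unless AffectCaster is set.
; Each tick applies the Gravity value as a mass-independent Z force to every target.
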(event OnComponentBeginOverlap(Sphere)
  (params (OverlappedComponent :type Primitive%20Component%20Object%20Reference) (OtherActor :type Actor%20Object%20Reference) (OtherComp :type Primitive%20Component%20Object%20Reference) (OtherBodyIndex :type Integer) (bFromSweep :type Boolean) (SweepResult :type Hit%20Result%20Structure%20%28by%20ref%29))
  (if (Math|Boolean|NANDBoolean (not (Variables|Settings-General|GetAffectCaster)) (== (Variables|Default|GetCharacter) OtherActor))
    (CallFunction|AddTarget OtherActor)))

(event OnComponentEndOverlap(Sphere)
  (params (OverlappedComponent :type Primitive%20Component%20Object%20Reference) (OtherActor :type Actor%20Object%20Reference) (OtherComp :type Primitive%20Component%20Object%20Reference) (OtherBodyIndex :type Integer))
  (CallFunction|RemoveTarget OtherActor))

(event Custom|RemoveTarget
  (params (Actor :type Actor%20Object%20Reference))
  (bind _telekinetic (CallFunction|IsTelekineticTarget Actor))
  (if _telekinetic
    (Utilities|Array|RemoveItem (Variables|Default|GetTargets) Actor)))

(event Custom|AddTarget
  (params (Actor :type Actor%20Object%20Reference))
  (bind _telekinetic (CallFunction|IsTelekineticTarget Actor))
  (if _telekinetic
    (Utilities|Array|Add (Variables|Default|GetTargets) Actor)))

(event EventBeginPlay
  (|CallParentFunction)
  (Transformation|SetActorLocation (Transformation|GetActorLocation (Variables|Default|GetCharacter)) false false)
  (Components|Sphere|SetSphereRadius (Variables|Components|GetSphere) (Variables|Settings-General|GetRadius) true)
  (Development|SetHiddeninGame (Variables|Components|GetSphere) (not (Variables|Default|GetDebug)) false))

(event EventTick
  (params (DeltaSeconds :type Float%20%28single-precision%29))
  (Utilities|FlowControl|Sequence
    (:then_0
      (if (Variables|Settings-General|GetFollowPlayer)
        (Transformation|SetActorLocation (Transformation|GetActorLocation (Variables|Default|GetCharacter)) true false)))
    (:then_1
      (for _array_element (Variables|Default|GetTargets)
        (CallFunction|AddForce _array_element (Math|Vector|MakeVector 0.0 0.0 (Variables|Settings-General|GetGravity)) "0, 0, 0" true)))))

(fn ConstructionScript
  (|CallParentFunction))