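; Telekinetic defense ability that slows nearby targets in front of the character.
; A sphere follows the character and tracks overlapping telekinetic targets other than the character.
; Each tick, targets within an aim cone, tested by dot product in 3D or flattened without pitch, receive impulses opposing their linear and angular velocity by a slow ratio.
; They also receive a vertical force set by Gravity.
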(event OnComponentBeginOverlap(Sphere)
  (params (OverlappedComponent :type Primitive%20Component%20Object%20Reference) (OtherActor :type Actor%20Object%20Reference) (OtherComp :type Primitive%20Component%20Object%20Reference) (OtherBodyIndex :type Integer) (bFromSweep :type Boolean) (SweepResult :type Hit%20Result%20Structure%20%28by%20ref%29))
  (if (not (== (Variables|Default|GetCharacter) OtherActor))
    (CallFunction|AddTarget OtherActor)))

(event OnComponentEndOverlap(Sphere)
  (params (OverlappedComponent :type Primitive%20Component%20Object%20Reference) (OtherActor :type Actor%20Object%20Reference) (OtherComp :type Primitive%20Component%20Object%20Reference) (OtherBodyIndex :type Integer))
  (CallFunction|RemoveTarget OtherActor))

(event Custom|RemoveTarget
  (params (Actor :type Actor%20Object%20Reference))
  (bind _telekinetic (CallFunction|IsTelekineticTarget Actor))
  (if _telekinetic
    (Utilities|Array|RemoveItem (Variables|Default|GetTargets) Actor)))

(event Custom|AddTarget
  (params (Actor :type Actor%20Object%20Reference))
  (bind _telekinetic (CallFunction|IsTelekineticTarget Actor))
  (if _telekinetic
    (Utilities|Array|Add (Variables|Default|GetTargets) Actor)))

(event EventBeginPlay
  (|CallParentFunction)
  (Variables|Settings-Defense|SetDefenseAngle (Math|Trig|Cos(Degrees) (/ (Variables|Settings-Defense|GetDefenseAngle) 2.0)))
  (Transformation|SetActorLocation (Transformation|GetActorLocation (Variables|Default|GetCharacter)) false false)
  (Components|Sphere|SetSphereRadius (Variables|Default|GetSphere) (Variables|Settings-Defense|GetRadius) true)
  (Development|SetHiddeninGame (Variables|Default|GetSphere) (not (Variables|Default|GetDebug)) false))

(event EventTick
  (params (DeltaSeconds :type Float%20%28single-precision%29))
  (bind _slowratio (Variables|Settings-Defense|GetSlowRatio))
  (bind _returnvalue (* _slowratio -1.0))
  (Utilities|FlowControl|Sequence
    (:then_0
      (Transformation|SetActorLocation (Transformation|GetActorLocation (Variables|Default|GetCharacter)) true false))
    (:then_1
      (for _array_element (Variables|Default|GetTargets)
        (Utilities|IsValid _array_element
          (:Is%20Valid
            (bind _dir (Class|BICaster|GetAim(Message) (Variables|Default|GetCharacter)))
            (if (>= (Math|Vector|DotProduct (Math|Vector|SelectVector _dir (Math|Vector|Normalize (* _dir "1.000000,1.000000, 0")) (Variables|Settings-Defense|GetPitch)) (Math|Vector|Normalize (Math|Vector|SelectVector (- (Transformation|GetActorLocation _array_element) (Transformation|GetActorLocation (Variables|Default|GetCharacter))) (* (- (Transformation|GetActorLocation _array_element) (Transformation|GetActorLocation (Variables|Default|GetCharacter))) "1.000000,1.000000, 0") (Variables|Settings-Defense|GetPitch)))) (Variables|Settings-Defense|GetDefenseAngle))
              (bind (_velocity _angularvelocity) (Class|BITarget|AbilityGetVel(Message) _array_element))
              (CallFunction|AddImpulse _array_element (* _velocity _returnvalue) (* _angularvelocity _returnvalue) true)
              (CallFunction|AddForce _array_element (Math|Vector|MakeVector 0.0 0.0 (Variables|Settings-Global|GetGravity)) "0, 0, 0" true))))))))

(fn ConstructionScript
  (|CallParentFunction))