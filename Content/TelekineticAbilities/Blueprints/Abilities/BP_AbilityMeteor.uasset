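; Telekinetic meteor ability that gathers objects along the character's aim, floats them above the character, then hurls them together at a target.
; While targeting, a timer loop runs multi-sphere traces, accumulating filtered hits in a deduplicating set mirrored to an array.
; Tick pulls gathered objects toward the float point with force.
; ShootMeteor aims by object trace, falling back to Visibility trace or maximum range, applies impulses, then clears targets.
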(event Custom|StopTargeting
  (Variables|Default|SetTargeting false))

(event Custom|TargetingHandler
  (if (Variables|Default|GetTargeting)
    (Utilities|FlowControl|Sequence
      (:then_0
        (bind (_origin _dir) (Class|BICaster|GetAim(Message) (Variables|Default|GetCharacter)))
        (bind _outhits (Collision|MultiSphereTraceForObjects (+ (* _dir (Variables|Settings-Targeting|GetAimRadius)) _origin) (+ _origin (* _dir (Variables|Settings-Targeting|GetAimRange))) (Variables|Settings-Targeting|GetAimRadius) (Variables|Settings-Targeting|GetTargetTypes) false (Utilities|Array|MakeArray (Variables|Default|GetCharacter)) (select (Variables|Default|GetDebug) "ForDuration" "None")))
        (bind _filtered (CallFunction|FilterHitTargets _outhits))
        (if (> (Utilities|Array|Length _filtered) 0)
          (CallFunction|AddTargets _filtered)))
      (:then_1
        (Utilities|Time|SetTimerbyEvent (delegate Custom|TargetingHandler) (Variables|Settings-Targeting|GetTargetingInterval))))))

(event Custom|StartTargeting
  (Variables|Default|SetTargeting true)
  (CallFunction|TargetingHandler))

(event Custom|ClearTargets
  (Utilities|Set|Clear (Variables|Default|GetTargetSet))
  (Utilities|Array|Clear (Variables|Default|GetTargetArray)))

(event EventBeginPlay
  (|CallParentFunction)
  (if (== (Variables|Settings-Targeting|GetTargetingInterval) 0.0)
    (Variables|Settings-Targeting|SetTargetingInterval 0.016667)))

(event EventTick
  (params (DeltaSeconds :type Float%20%28single-precision%29))
  (for _array_element (Variables|Default|GetTargetArray)
    (CallFunction|AddForceToward (+ (Transformation|GetActorLocation (Variables|Default|GetCharacter)) (Math|Vector|MakeVector 0.0 0.0 (Variables|Settings-Float|GetFloatHeight))) _array_element (Variables|Settings-Float|GetFloatSpeedMultiplier) (Variables|Settings-Float|GetFloatAngularReduction) (Variables|Settings-Global|GetGravity))))

(fn ConstructionScript
  (|CallParentFunction))

(fn AddTargets
  (params (Targets :type Array%20of%20Actor%20Object%20References))
  (LocalVariables|SetCount (Utilities|Set|Length (Variables|Default|GetTargetSet)))
  (for _array_element Targets
    (Utilities|Set|Add (Variables|Default|GetTargetSet) _array_element))
  (if (!= (Utilities|Set|Length (Variables|Default|GetTargetSet)) (LocalVariables|GetCount))
    (bind _result (Utilities|Set|ToArray (Variables|Default|GetTargetSet)))
    (Variables|Default|SetTargetArray _result)))

(fn ShootMeteor
  (bind _output_get (LocalVariables|SetIgnore (Variables|Default|GetTargetArray)))
  (Utilities|Array|Add _output_get (Variables|Default|GetCharacter))
  (Utilities|FlowControl|Sequence
    (:then_0
      (bind (_origin _dir) (Class|BICaster|GetAim(Message) (Variables|Default|GetCharacter)))
      (bind (_outhit _returnvalue) (Collision|SphereTraceForObjects (+ (* _dir (Variables|Settings-Shoot|GetShootAimRadius)) _origin) (+ _origin (* _dir (Variables|Settings-Shoot|GetShootAimRange))) (Variables|Settings-Shoot|GetShootAimRadius) (Variables|Settings-Shoot|GetShootTargetTypes) false (LocalVariables|GetIgnore) (select (Variables|Default|GetDebug) "ForDuration" "None")))
      (if _returnvalue
        (LocalVariables|SettTarget (Transformation|GetActorLocation (.HitActor (Collision|BreakHitResult _outhit))))
        (else
          (bind (_outhit_2 _returnvalue_2) (Collision|SphereTraceByChannel (.TraceStart (Collision|BreakHitResult _outhit)) (.TraceEnd (Collision|BreakHitResult _outhit)) (Variables|Settings-Shoot|GetShootAimRadius) "TraceTypeQuery1" false (LocalVariables|GetIgnore) (select (Variables|Default|GetDebug) "ForDuration" "None") true "(R=1.000000,G=0.453602,B=0.000000,A=1.000000)" "(R=0.000000,G=0.702205,B=1.000000,A=1.000000)"))
          (if _returnvalue_2
            (LocalVariables|SettTarget (.Location (Collision|BreakHitResult _outhit_2)))
            (else
              (LocalVariables|SettTarget (.TraceEnd (Collision|BreakHitResult _outhit_2))))))))
    (:then_1
      (for _array_element (Variables|Default|GetTargetArray)
        (CallFunction|AddImpulseToward _array_element (LocalVariables|GettTarget) (Variables|Settings-Shoot|GetShootForce) 9.8e+02)))
    (:then_2
      (CallFunction|ClearTargets))))