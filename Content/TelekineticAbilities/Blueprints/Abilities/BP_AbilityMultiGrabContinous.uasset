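; Telekinetic multi-grab ability that gathers objects along the character's aim, then holds them in front of the player.
; From BeginPlay, a self-rescheduling timer repeats sphere traces, adding filtered hits to a deduplicating set mirrored into an array for iteration.
; Once targeting stops, Tick continuously applies force pulling each target toward a hold point along the current aim, optionally offset by player velocity.
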(event Custom|StopTargeting
  (Variables|Default|SetTargeting false))

(event Custom|TargetingHandler
  (if (Variables|Default|GetTargeting)
    (Utilities|FlowControl|Sequence
      (:then_0
        (bind (_origin _dir) (Class|BICaster|GetAim(Message) (Variables|Default|GetCharacter)))
        (bind _outhits (Collision|MultiSphereTraceForObjects (+ (* _dir (Variables|Settings-Aim|GetAimRadius)) _origin) (+ _origin (* _dir (Variables|Settings-Aim|GetAimRange))) (Variables|Settings-Aim|GetAimRadius) (Variables|Settings-Aim|GetTargetTypes) false (Utilities|Array|MakeArray (Variables|Default|GetCharacter)) (select (Variables|Default|GetDebug) "ForDuration" "None")))
        (bind _filtered (CallFunction|FilterHitTargets _outhits))
        (if (> (Utilities|Array|Length _filtered) 0)
          (CallFunction|AddTargets _filtered)))
      (:then_1
        (Utilities|Time|SetTimerbyEvent (delegate Custom|TargetingHandler) (Variables|Settings-Aim|GetTargetingInterval))))))

(event Custom|StartTargeting
  (CallFunction|ClearTargets)
  (Variables|Default|SetTargeting true)
  (CallFunction|TargetingHandler))

(event Custom|ClearTargets
  (Utilities|Set|Clear (Variables|Default|GetTargetSet))
  (Utilities|Array|Clear (Variables|Default|GetTargetArray)))

(event EventBeginPlay
  (|CallParentFunction)
  (CallFunction|SetDefaultFloatValue (Variables|Settings-Aim|GetTargetingInterval) 0.033333)
  (CallFunction|StartTargeting))

(event EventTick
  (params (DeltaSeconds :type Float%20%28single-precision%29))
  (bind _character (Variables|Default|GetCharacter))
  (if (not (Variables|Default|GetTargeting))
    (for _array_element (Variables|Default|GetTargetArray)
      (bind (_origin _dir) (Class|BICaster|GetAim(Message) _character))
      (CallFunction|AddForceToward (+ _origin (* _dir (Variables|Settings-Hold|GetHoldRange)) (Math|Vector|SelectVector (Transformation|GetVelocity _character) "0, 0, 0" (Variables|Settings-Hold|GetConsiderPlayerVelocity))) _array_element (Variables|Settings-Hold|GetHoldSpeedMultiplier) (Variables|Settings-Hold|GetHoldAngularReduction) (Variables|Settings-Global|GetGravity)))))

(fn ConstructionScript
  (|CallParentFunction))

(fn AddTargets
  (params (Targets :type Array%20of%20Actor%20Object%20References))
  (LocalVariables|SetCount (Utilities|Set|Length (Variables|Default|GetTargetSet)))
  (for _array_element Targets
    (Utilities|Set|Add (Variables|Default|GetTargetSet) _array_element))
  (if (!= (Utilities|Set|Length (Variables|Default|GetTargetSet)) (LocalVariables|GetCount))
    (bind _result (Utilities|Set|ToArray (Variables|Default|GetTargetSet)))
    (Variables|Default|SetTargetArray _result)))