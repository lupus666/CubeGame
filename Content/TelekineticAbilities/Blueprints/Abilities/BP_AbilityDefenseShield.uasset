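; Telekinetic defense shield ability actor that pulls nearby telekinetic objects into an orbit around the character.
; It follows the character each tick, and its sphere overlap registers valid targets, never removing them.
; Each target's horizontal approach direction is stored in the rotating frame at orbit radius.
; Every tick the angle advances and Shielding pushes targets toward their rotated slots, leading by character velocity.
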(event OnComponentBeginOverlap(Sphere)
  (params (OverlappedComponent :type Primitive%20Component%20Object%20Reference) (OtherActor :type Actor%20Object%20Reference) (OtherComp :type Primitive%20Component%20Object%20Reference) (OtherBodyIndex :type Integer) (bFromSweep :type Boolean) (SweepResult :type Hit%20Result%20Structure%20%28by%20ref%29))
  (if (not (== OtherActor (Variables|Default|GetCharacter)))
    (bind _telekinetic (CallFunction|IsTelekineticTarget OtherActor))
    (if _telekinetic
      (CallFunction|AddTarget OtherActor))))

(event Custom|AddTarget
  (params (Actor :type Actor%20Object%20Reference))
  (Utilities|Array|Add (Variables|Default|GetTargets) Actor)
  (Utilities|Array|Add (Variables|Default|GetOffsets) (* (Math|Vector|Normalize (Math|Vector|UnrotateVector (* (- (Transformation|GetActorLocation Actor) (Transformation|GetActorLocation (Variables|Default|GetCharacter))) "1.000000,1.000000, 0") (Math|Rotator|MakeRotator 0.0 0.0 (Variables|Default|GetOffset)))) (Variables|Settings-Defense|GetOrbitingRadius))))

(event EventBeginPlay
  (|CallParentFunction)
  (Transformation|SetActorLocation (Transformation|GetActorLocation (Variables|Default|GetCharacter)) false false)
  (Components|Sphere|SetSphereRadius (Variables|Default|GetSphere) (Variables|Settings-Defense|GetRadius) true)
  (Development|SetHiddeninGame (Variables|Default|GetSphere) (not (Variables|Default|GetDebug)) false))

(event EventTick
  (params (DeltaSeconds :type Float%20%28single-precision%29))
  (Utilities|FlowControl|Sequence
    (:then_0
      (Transformation|SetActorLocation (Transformation|GetActorLocation (Variables|Default|GetCharacter)) true false))
    (:then_1
      (Variables|Default|SetOffset (Math|Float|%(Float) (+ (* DeltaSeconds (Variables|Settings-Defense|GetOrbitingSpeed)) (Variables|Default|GetOffset)) 3.6e+02))
      (CallFunction|Shielding))))

(fn ConstructionScript
  (|CallParentFunction))

(fn Shielding
  (bind _character (Variables|Default|GetCharacter))
  (for (_array_element _array_index) (Variables|Default|GetTargets)
    (Utilities|IsValid _array_element
      (:Is%20Valid
        (Class|BITarget|AbilityGetVel(Message) _array_element)
        (CallFunction|AddForceToward (+ (Math|Vector|RotateVector (Utilities|Array|Get(acopy) (Variables|Default|GetOffsets) _array_index) (Math|Rotator|MakeRotator 0.0 0.0 (Variables|Default|GetOffset))) (Transformation|GetActorLocation _character) (Transformation|GetVelocity _character)) _array_element 1e+01 0.1 9.8e+02)))))