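; Telekinetic black hole ability that spawns at a set distance along the character's aim and pulls nearby targets toward its center.
; A sphere grows from start to end radius over time, and its overlaps maintain the list of telekinetic targets, excluding the caster.
; Each tick, targets within the radius receive a mass-independent force with exponential-power distance falloff, plus a vertical gravity term when Weightless is set.
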(event OnComponentBeginOverlap(Sphere)
  (params (OverlappedComponent :type Primitive%20Component%20Object%20Reference) (OtherActor :type Actor%20Object%20Reference) (OtherComp :type Primitive%20Component%20Object%20Reference) (OtherBodyIndex :type Integer) (bFromSweep :type Boolean) (SweepResult :type Hit%20Result%20Structure%20%28by%20ref%29))
  (if (not (== (Variables|Default|GetCharacter) OtherActor))
    (CallFunction|AddTarget OtherActor)))

(event OnComponentEndOverlap(Sphere)
  (params (OverlappedComponent :type Primitive%20Component%20Object%20Reference) (OtherActor :type Actor%20Object%20Reference) (OtherComp :type Primitive%20Component%20Object%20Reference) (OtherBodyIndex :type Integer))
  (CallFunction|RemoveTarget OtherActor))

(event Custom|RemoveTarget
  (params (Actor :type Actor%20Object%20Reference))
  (bind _telekinetic (CallFunction|IsTelekineticTarget Actor))
  (if _telekinetic
    (Utilities|Array|RemoveItem (Variables|Default|GetTargets) Actor)))

(event Custom|AddTarget
  (params (Actor :type Actor%20Object%20Reference))
  (bind _telekinetic (CallFunction|IsTelekineticTarget Actor))
  (if _telekinetic
    (Utilities|Array|Add (Variables|Default|GetTargets) Actor)))

(event EventBeginPlay
  (|CallParentFunction)
  (bind (_origin _dir) (Class|BICaster|GetAim(Message) (Variables|Default|GetCharacter)))
  (Transformation|SetActorLocation (+ _origin (* _dir (Variables|Settings-Aim|GetAimDistance))) false false)
  (Components|Sphere|SetSphereRadius (Variables|Default|GetSphere) (Variables|Settings-Size|GetStartRadius) true)
  (Development|SetHiddeninGame (Variables|Default|GetSphere) (not (Variables|Default|GetDebug)) false))

(event EventTick
  (params (DeltaSeconds :type Float%20%28single-precision%29))
  (Utilities|FlowControl|Sequence
    (:then_0
      (Variables|Default|SetGrowth (Math|Float|Min(Float) (+ (Variables|Default|GetGrowth) DeltaSeconds) (Variables|Settings-Size|GetGrowTime)))
      (Components|Sphere|SetSphereRadius (Variables|Default|GetSphere) (Math|Float|Lerp (Variables|Settings-Size|GetStartRadius) (Variables|Settings-Size|GetEndRadius) (/ (Variables|Default|GetGrowth) (Variables|Settings-Size|GetGrowTime))) true))
    (:then_1
      (CallFunction|PullTowardsBlackHole))))

(fn ConstructionScript
  (|CallParentFunction))

(fn PullTowardsBlackHole
  (LocalVariables|SetRadius (Math|Float|Lerp (Variables|Settings-Size|GetStartRadius) (Variables|Settings-Size|GetEndRadius) (/ (Variables|Default|GetGrowth) (Variables|Settings-Size|GetGrowTime))))
  (for _array_element (Variables|Default|GetTargets)
    (Utilities|IsValid _array_element
      (:Is%20Valid
        (if (< (Transformation|GetDistanceTo _array_element self) (LocalVariables|GetRadius))
          (CallFunction|AddForce _array_element (+ (* (Math|Vector|Normalize (- (Transformation|GetActorLocation) (Transformation|GetActorLocation _array_element))) (* (Math|Float|Power (- 1.0 (/ (Transformation|GetDistanceTo _array_element self) (LocalVariables|GetRadius))) (Variables|Settings-Force|GetForceDistanceExponent)) (Variables|Settings-Force|GetForce))) (Math|Vector|SelectVector (Math|Vector|MakeVector 0.0 0.0 (Variables|Settings-Global|GetGravity)) "0, 0, 0" (Variables|Settings-Force|GetWeightless))) "0, 0, 0" true))))))