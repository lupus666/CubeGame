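; Telekinetic crush ability actor that pulls surrounding objects toward an aimed point, then destroys itself.
; On BeginPlay, GetTargets sphere-traces along the character's aim for an object, falling back to a visibility hit or trace end.
; It gathers filtered actors in a charge-scaled sphere there, excluding the character and aimed actor.
; Each gets an impulse toward the center, optionally scaled by distance, with optional debug drawing.
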(event EventBeginPlay
  (|CallParentFunction)
  (bind (_actors _target) (CallFunction|GetTargets))
  (for _array_element _actors
    (CallFunction|AddImpulsewithForce _array_element (* (Math|Vector|Normalize (- _target (Transformation|GetActorLocation _array_element))) (Math|Float|SelectFloat (/ (Math|Vector|VectorLength (- _target (Transformation|GetActorLocation _array_element))) (CallFunction|ChargeLerp (Variables|Settings-Force|GetMinRange) (Variables|Settings-Force|GetMaxRange))) 1.0 (Variables|Settings-Force|GetDistanceAffectForce)))))
  (Actor|DestroyActor))

(fn ConstructionScript
  (|CallParentFunction))

(fn GetTargets
  (Utilities|FlowControl|Sequence
    (:then_0
      (bind (_origin _dir) (Class|BICaster|GetAim(Message) (Variables|Default|GetCharacter)))
      (bind (_outhit _returnvalue) (Collision|SphereTraceForObjects (+ (* _dir (Variables|Settings-Aim|GetAimRadius)) _origin) (+ _origin (* _dir (CallFunction|ChargeLerp (Variables|Settings-Aim|GetMinAimRange) (Variables|Settings-Aim|GetMaxAimRange)))) (Variables|Settings-Aim|GetAimRadius) (Variables|Settings-Aim|GetAimTypes) false (Utilities|Array|MakeArray (Variables|Default|GetCharacter)) (select (Variables|Default|GetDebug) "ForDuration" "None")))
      (if _returnvalue
        (LocalVariables|SettTarget (Transformation|GetActorLocation (.HitActor (Collision|BreakHitResult _outhit))))
        (LocalVariables|SettTargetActor (.HitActor (Collision|BreakHitResult _outhit)))
        (else
          (bind (_outhit_2 _returnvalue_2) (Collision|SphereTraceByChannel (.TraceStart (Collision|BreakHitResult _outhit)) (.TraceEnd (Collision|BreakHitResult _outhit)) (Variables|Settings-Aim|GetAimRadius) "TraceTypeQuery1" false (Utilities|Array|MakeArray (Variables|Default|GetCharacter)) (select (Variables|Default|GetDebug) "ForDuration" "None") true "(R=1.000000,G=0.453602,B=0.000000,A=1.000000)" "(R=0.000000,G=0.702205,B=1.000000,A=1.000000)"))
          (if _returnvalue_2
            (LocalVariables|SettTarget (.Location (Collision|BreakHitResult _outhit_2)))
            (else
              (LocalVariables|SettTarget (.TraceEnd (Collision|BreakHitResult _outhit_2))))))))
    (:then_1
      (Utilities|FlowControl|Sequence
        (:then_0
          (if (Variables|Default|GetDebug)
            (Rendering|Debug|DrawDebugSphere (LocalVariables|GettTarget) (CallFunction|ChargeLerp (Variables|Settings-Force|GetMinRange) (Variables|Settings-Force|GetMaxRange)) 16 "(R=1.000000,G=0.148011,B=0.000000,A=1.000000)" 5.0 2.0)))
        (:then_1
          (bind _outactors (Collision|SphereOverlapActors (LocalVariables|GettTarget) (CallFunction|ChargeLerp (Variables|Settings-Force|GetMinRange) (Variables|Settings-Force|GetMaxRange)) (Variables|Settings-Force|GetTargetTypes) 0 (Utilities|Array|MakeArray (Variables|Default|GetCharacter) (LocalVariables|GettTargetActor))))
          (bind _filtered (CallFunction|FilterTargets _outactors))
          (return _filtered (LocalVariables|GettTarget)))))))