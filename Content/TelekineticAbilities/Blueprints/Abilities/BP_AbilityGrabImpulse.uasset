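; Telekinetic grab ability that flings an aimed object toward a drop point in front of the character with one impulse.
; On BeginPlay, a sphere trace along the character's aim finds a telekinetic target and passes it to Pull.
; Pull solves a ballistic launch velocity from drop time and gravity, optionally leading for character movement.
; The mass-independent impulse subtracts the target's current velocity and counters its spin.
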(event Custom|Pull
  (params (Actor :type Actor%20Object%20Reference))
  (bind _character (Variables|Default|GetCharacter))
  (bind _dir (Class|BICaster|GetAim(Message) (Variables|Default|GetCharacter)))
  (bind (_velocity _angularvelocity) (CallFunction|GetTargetVelocity Actor))
  (CallFunction|AddImpulse Actor (- (+ (/ (- (+ (* _dir (Variables|Settings-Drop|GetDropRange)) (Transformation|GetActorLocation _character) (Math|Vector|SelectVector (* (Transformation|GetVelocity _character) (Variables|Settings-Drop|GetDropTime)) "0, 0, 0" (Variables|Settings-Drop|GetConsiderPlayerVelocity))) (Transformation|GetActorLocation Actor)) (Variables|Settings-Drop|GetDropTime)) (Math|Vector|MakeVector 0.0 0.0 (* (* (Variables|Settings-Drop|GetDropTime) 0.5) (Variables|Settings-Global|GetGravity)))) _velocity) (* _angularvelocity -1.0) true))

(event EventBeginPlay
  (|CallParentFunction)
  (bind (_found _target) (CallFunction|GetTarget))
  (if _found
    (CallFunction|Pull _target)))

(fn ConstructionScript
  (|CallParentFunction))

(fn GetTarget
  (bind (_origin _dir) (Class|BICaster|GetAim(Message) (Variables|Default|GetCharacter)))
  (bind (_outhit _returnvalue) (Collision|SphereTraceForObjects (+ (* _dir (Variables|Settings-Aim|GetAimRadius)) _origin) (+ _origin (* _dir (Variables|Settings-Aim|GetAimRange))) (Variables|Settings-Aim|GetAimRadius) (Variables|Settings-Aim|GetTargetTypes) false (Utilities|Array|MakeArray (Variables|Default|GetCharacter)) (select (Variables|Default|GetDebug) "ForDuration" "None")))
  (if _returnvalue
    (bind _telekinetic (CallFunction|IsTelekineticTarget (.HitActor (Collision|BreakHitResult _outhit))))
    (if _telekinetic
      (return true (.HitActor (Collision|BreakHitResult _outhit))))))