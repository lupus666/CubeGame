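; Telekinetic push ability actor that shoves targets in front of its Character along the aim direction, then destroys itself on BeginPlay.
; A zero-length box trace, sized by Charge and offset half its depth along the aim, gathers objects of the target types, which are then filtered.
; Each target receives an impulse along the aim vector, and the Pitch flag decides whether that impulse and the box orientation keep their vertical component.
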(event Custom|Push
  (params (Targets :type Array%20of%20Actor%20Object%20References))
  (for _array_element Targets
    (bind _dir (Class|BICaster|GetAim(Message) (Variables|Default|GetCharacter)))
    (CallFunction|AddImpulsewithForce _array_element (Math|Vector|SelectVector _dir (* _dir "1.000000,1.000000, 0") (Variables|Settings-Force|GetPitch)))))

(event EventBeginPlay
  (|CallParentFunction)
  (bind _actors (CallFunction|GetTargets))
  (CallFunction|Push _actors)
  (Actor|DestroyActor))

(fn ConstructionScript
  (|CallParentFunction))

(fn GetTargets
  (LocalVariables|SetBox (Math|Vector|Lerp(Vector) (Variables|Settings-Targeting|GetMinBox) (Variables|Settings-Targeting|GetMaxBox) (Variables|Default|GetCharge)))
  (bind _dir (Class|BICaster|GetAim(Message) (Variables|Default|GetCharacter)))
  (bind _outhits (Class|KismetSystemLibrary|BoxTraceMultiforObjects (+ (* _dir (* (.X (Math|Vector|BreakVector (LocalVariables|GetBox))) 0.5)) (Transformation|GetActorLocation (Variables|Default|GetCharacter))) (+ (* _dir (* (.X (Math|Vector|BreakVector (LocalVariables|GetBox))) 0.5)) (Transformation|GetActorLocation (Variables|Default|GetCharacter))) (* (LocalVariables|GetBox) 0.5) (Math|Conversions|RotationFromXVector (Math|Vector|SelectVector _dir (* _dir "1.000000,1.000000, 0") (Variables|Settings-Force|GetPitch))) (Variables|Settings-Targeting|GetTargetTypes) false (Utilities|Array|MakeArray (Variables|Default|GetCharacter)) (select (Variables|Default|GetDebug) "ForDuration" "None") true))
  (bind _filtered (CallFunction|FilterHitTargets _outhits))
  (return _filtered))