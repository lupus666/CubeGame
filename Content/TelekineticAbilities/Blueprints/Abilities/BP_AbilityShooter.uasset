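; Telekinetic shooter ability that grabs objects the character aims at, holds them afloat and launches them at targets.
; FindTarget sphere-traces along the aim and adds valid telekinetic actors, up to a maximum count.
; Each tick, forces pull held objects toward ring slots above the character, rotated with aim yaw and offset by velocity.
; ShootTarget releases the oldest with an impulse toward a traced target, falling back to visibility hit or trace end.
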(event Custom|AddTarget
  (params (Target :type Actor%20Object%20Reference))
  (if (> (Variables|Settings-Float|GetMaxObjects) (Utilities|Array|Length (Variables|Default|GetObjects)))
    (Utilities|Array|AddUnique (Variables|Default|GetObjects) Target)))

(event EventTick
  (params (DeltaSeconds :type Float%20%28single-precision%29))
  (CallFunction|FloatObjects))

(fn ConstructionScript
  (|CallParentFunction))

(fn FloatObjects
  (bind _floatradius (Variables|Settings-Float|GetFloatRadius))
  (bind _character (Variables|Default|GetCharacter))
  (for (_array_element _array_index) (Variables|Default|GetObjects)
    (bind _output_get (LocalVariables|SetObject _array_element))
    (Utilities|IsValid _output_get
      (:Is%20Valid
        (LocalVariables|SetRad (* (/ (Math|Conversions|ToFloat(Integer) _array_index) (Math|Conversions|ToFloat(Integer) (Variables|Settings-Float|GetMaxObjects))) (Math|Trig|GetPI) 2.0))
        (bind _dir (Class|BICaster|GetAim(Message) (Variables|Default|GetCharacter)))
        (bind _output_get_2 (LocalVariables|SetTarget (Math|Vector|RotateVector (Math|Vector|MakeVector (* (Math|Trig|Cos(Radians) (LocalVariables|GetRad)) _floatradius) (* _floatradius (Math|Trig|Sin(Radians) (LocalVariables|GetRad))) (Variables|Settings-Float|GetFloatHeight)) (Math|Rotator|MakeRotator 0.0 0.0 (.Yaw (Math|Rotator|BreakRotator (Math|Conversions|RotationFromXVector _dir)))))))
        (CallFunction|AddForceToward (+ _output_get_2 (Transformation|GetActorLocation _character) (Transformation|GetVelocity _character)) (LocalVariables|GetObject) (Variables|Settings-Float|GetFloatSpeedMultiplier) 0.1 (Variables|Settings-Global|GetGravity))))))

(fn ShootTarget
  (if (> (Utilities|Array|Length (Variables|Default|GetObjects)) 0)
    (bind _output_get (LocalVariables|SetIgnore (Variables|Default|GetObjects)))
    (Utilities|Array|Add _output_get (Variables|Default|GetCharacter))
    (LocalVariables|SetBullet (Utilities|Array|Get(acopy) (Variables|Default|GetObjects)))
    (Utilities|Array|RemoveIndex (Variables|Default|GetObjects))
    (Utilities|FlowControl|Sequence
      (:then_0
        (bind (_origin _dir) (Class|BICaster|GetAim(Message) (Variables|Default|GetCharacter)))
        (bind (_outhit _returnvalue) (Collision|SphereTraceForObjects (+ (* _dir (Variables|Settings-Shoot|GetShootAimRadius)) _origin) (+ _origin (* _dir (Variables|Settings-Shoot|GetShootAimRange))) (Variables|Settings-Shoot|GetShootAimRadius) (Variables|Settings-Shoot|GetShootTargetTypes) false (LocalVariables|GetIgnore) (select (Variables|Default|GetDebug) "ForDuration" "None")))
        (if _returnvalue
          (LocalVariables|SettTarget (Transformation|GetActorLocation (.HitActor (Collision|BreakHitResult _outhit))))
          (else
            (bind (_outhit_2 _returnvalue_2) (Collision|SphereTraceByChannel (.TraceStart (Collision|BreakHitResult _outhit)) (.TraceEnd (Collision|BreakHitResult _outhit)) (Variables|Settings-Shoot|GetShootAimRadius) "TraceTypeQuery1" false (LocalVariables|GetIgnore) (select (Variables|Default|GetDebug) "ForDuration" "None") true "(R=1.000000,G=0.453602,B=0.000000,A=1.000000)" "(R=0.000000,G=0.702205,B=1.000000,A=1.000000)"))
            (if _returnvalue_2
              (LocalVariables|SettTarget (.Location (Collision|BreakHitResult _outhit_2)))
              (else
                (LocalVariables|SettTarget (.TraceEnd (Collision|BreakHitResult _outhit_2))))))))
      (:then_1
        (CallFunction|AddImpulseToward (LocalVariables|GetBullet) (LocalVariables|GettTarget) (Variables|Settings-Shoot|GetShootForce) 9.8e+02)))))

(fn FindTarget
  (bind _output_get (LocalVariables|SetIgnore (Variables|Default|GetObjects)))
  (Utilities|Array|Add _output_get (Variables|Default|GetCharacter))
  (bind (_origin _dir) (Class|BICaster|GetAim(Message) (Variables|Default|GetCharacter)))
  (bind (_outhit _returnvalue) (Collision|SphereTraceForObjects (+ (* _dir (Variables|Settings-Targeting|GetAimRadius)) _origin) (+ _origin (* _dir (Variables|Settings-Targeting|GetAimRange))) (Variables|Settings-Targeting|GetAimRadius) (Variables|Settings-Targeting|GetTargetTypes) false (LocalVariables|GetIgnore) (select (Variables|Default|GetDebug) "ForDuration" "None")))
  (if _returnvalue
    (bind _telekinetic (CallFunction|IsTelekineticTarget (.HitActor (Collision|BreakHitResult _outhit))))
    (if _telekinetic
      (CallFunction|AddTarget (.HitActor (Collision|BreakHitResult _outhit))))))