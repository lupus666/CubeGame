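; Telekinetic radial push ability that shoves nearby targets away from the casting character within a cone around the aim direction.
; On BeginPlay the authority gathers filtered targets with a sphere overlap, pushes them once and destroys the actor.
; Charge scales both radius and cone angle, with half-angles pre-converted to cosines for a dot-product test.
; The Pitch flag chooses between 3D and horizontal-only aim and push directions.
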(event EventBeginPlay
  (|CallParentFunction)
  (Variables|Settings-Targeting|SetMinAngle (Math|Trig|Cos(Degrees) (/ (Variables|Settings-Targeting|GetMinAngle) 2.0)))
  (Variables|Settings-Targeting|SetMaxAngle (Math|Trig|Cos(Degrees) (/ (Variables|Settings-Targeting|GetMaxAngle) 2.0)))
  (Networking|SwitchHasAuthority
    (:Authority
      (bind _actors (CallFunction|GetTargets))
      (CallFunction|RadialPush _actors)
      (Actor|DestroyActor))))

(fn ConstructionScript
  (|CallParentFunction))

(fn GetTargets
  (Utilities|FlowControl|Sequence
    (:then_0
      (if (Variables|Default|GetDebug)
        (Rendering|Debug|DrawDebugSphere (Transformation|GetActorLocation (Variables|Default|GetCharacter)) (CallFunction|ChargeLerp (Variables|Settings-Targeting|GetMinRange) (Variables|Settings-Targeting|GetMaxRange)) 16 "(R=1.000000,G=0.148011,B=0.000000,A=1.000000)" 5.0 2.0)))
    (:then_1
      (bind _outactors (Collision|SphereOverlapActors (Transformation|GetActorLocation (Variables|Default|GetCharacter)) (CallFunction|ChargeLerp (Variables|Settings-Targeting|GetMinRange) (Variables|Settings-Targeting|GetMaxRange)) (Variables|Settings-Targeting|GetTargetTypes) 0 (Utilities|Array|MakeArray (Variables|Default|GetCharacter))))
      (bind _filtered (CallFunction|FilterTargets _outactors))
      (return _filtered))))

(fn RadialPush
  (params (Actors :type Array%20of%20Actor%20Object%20References))
  (for _array_element Actors
    (LocalVariables|SetTarget _array_element)
    (bind _dir (Class|BICaster|GetAim(Message) (Variables|Default|GetCharacter)))
    (if (>= (Math|Vector|DotProduct (Math|Vector|SelectVector _dir (Math|Vector|Normalize (* _dir "1.000000,1.000000, 0")) (Variables|Settings-Targeting|GetPitch)) (Math|Vector|Normalize (Math|Vector|SelectVector (- (Transformation|GetActorLocation _array_element) (Transformation|GetActorLocation (Variables|Default|GetCharacter))) (* (- (Transformation|GetActorLocation _array_element) (Transformation|GetActorLocation (Variables|Default|GetCharacter))) "1.000000,1.000000, 0") (Variables|Settings-Targeting|GetPitch)))) (CallFunction|ChargeLerp (Variables|Settings-Targeting|GetMinAngle) (Variables|Settings-Targeting|GetMaxAngle)))
      (CallFunction|AddImpulsewithForce (LocalVariables|GetTarget) (Math|Vector|Normalize (Math|Vector|SelectVector (- (Transformation|GetActorLocation _array_element) (Transformation|GetActorLocation (Variables|Default|GetCharacter))) (* (- (Transformation|GetActorLocation _array_element) (Transformation|GetActorLocation (Variables|Default|GetCharacter))) "1.000000,1.000000, 0") (Variables|Settings-Targeting|GetPitch)))))))