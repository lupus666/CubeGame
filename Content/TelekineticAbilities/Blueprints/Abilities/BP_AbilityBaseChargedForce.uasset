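; Base telekinetic ability whose force depends on charge, judging by its name and charge interpolation helper.
; On BeginPlay, after the parent logic, it passes Force with its minimum and maximum bounds to ChargeLerpVar.
; AddImpulseWithForce scales a given base vector by Force and applies it to a target as an impulse, optionally ignoring mass.
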(event EventBeginPlay
  (|CallParentFunction)
  (CallFunction|ChargeLerpVar (Variables|Default|GetForce) (Variables|Settings-Force|GetMinForce) (Variables|Settings-Force|GetMaxForce)))

(fn ConstructionScript
  (|CallParentFunction))

(fn AddImpulsewithForce
  (params (Target :type Actor%20Object%20Reference) (Base :type Vector))
  (CallFunction|AddImpulse Target (* Base (Variables|Default|GetForce)) "0, 0, 0" (Variables|Settings-Force|GetIgnoreMass)))