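; BP_AbilityPull is a telekinetic ability that pulls targets toward the owning character as soon as it begins play.
; It sphere-traces along the character's aim over a charge-interpolated range and filters the hits into valid targets.
; Each target receives an impulse toward the character, optionally scaled by its distance relative to that range, so farther targets are pulled harder.
; An optional debug flag draws the trace.
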(event Custom|Pull
  (params (Actors :type Array%20of%20Actor%20Object%20References))
  (for _array_element Actors
    (CallFunction|AddImpulsewithForce _array_element (* (Math|Vector|Normalize (- (Transformation|GetActorLocation (Variables|Default|GetCharacter)) (Transformation|GetActorLocation _array_element))) (Math|Float|SelectFloat (/ (Math|Vector|VectorLength (- (Transformation|GetActorLocation (Variables|Default|GetCharacter)) (Transformation|GetActorLocation _array_element))) (CallFunction|ChargeLerp (Variables|Settings-Aim|GetMinAimRange) (Variables|Settings-Aim|GetMaxAimRange))) 1.0 (Variables|Settings-Force|GetDistanceAffectForce))))))

(event EventBeginPlay
  (|CallParentFunction)
  (bind _targets (CallFunction|GetTargets))
  (CallFunction|Pull _targets))

(fn ConstructionScript
  (|CallParentFunction))

(fn GetTargets
  (bind (_origin _dir) (Class|BICaster|GetAim(Message) (Variables|Default|GetCharacter)))
  (bind _outhits (Collision|MultiSphereTraceForObjects _origin (+ _origin (* _dir (CallFunction|ChargeLerp (Variables|Settings-Aim|GetMinAimRange) (Variables|Settings-Aim|GetMaxAimRange)))) (Variables|Settings-Aim|GetAimRadius) (Variables|Settings-Aim|GetTargetTypes) false (Utilities|Array|MakeArray (Variables|Default|GetCharacter)) (select (Variables|Default|GetDebug) "ForDuration" "None")))
  (bind _filtered (CallFunction|FilterHitTargets _outhits))
  (return _filtered))