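; Continuous telekinetic grab ability that holds an object in front of the character's aim.
; On BeginPlay it sphere-traces along the aim ray and stores the hit actor as Target if it is a telekinetic target.
; Each Tick it applies force pulling Target toward a point at hold range along the current aim, optionally offset by player velocity, with angular reduction and gravity parameters.
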(event Custom|SetTarget
  (params (Target :type Actor%20Object%20Reference))
  (Variables|Default|SetTarget Target))

(event Custom|ClearTarget
  (Variables|Default|SetTarget 0))

(event Custom|FindTarget
  (bind (_origin _dir) (Class|BICaster|GetAim(Message) (Variables|Default|GetCharacter)))
  (bind (_outhit _returnvalue) (Collision|SphereTraceForObjects (+ (* _dir (Variables|Settings-Aim|GetAimRadius)) _origin) (+ _origin (* _dir (Variables|Settings-Aim|GetAimRange))) (Variables|Settings-Aim|GetAimRadius) (Variables|Settings-Aim|GetTargetTypes) false (Utilities|Array|MakeArray (Variables|Default|GetCharacter)) (select (Variables|Default|GetDebug) "ForDuration" "None")))
  (if _returnvalue
    (bind _telekinetic (CallFunction|IsTelekineticTarget (.HitActor (Collision|BreakHitResult _outhit))))
    (if _telekinetic
      (CallFunction|SetTarget (.HitActor (Collision|BreakHitResult _outhit))))))

(event EventBeginPlay
  (|CallParentFunction)
  (CallFunction|FindTarget))

(event EventTick
  (params (DeltaSeconds :type Float%20%28single-precision%29))
  (bind _character (Variables|Default|GetCharacter))
  (Utilities|IsValid (Variables|Default|GetTarget)
    (:Is%20Valid
      (bind (_origin _dir) (Class|BICaster|GetAim(Message) _character))
      (CallFunction|AddForceToward (+ _origin (* _dir (Variables|Settings-Hold|GetHoldRange)) (Math|Vector|SelectVector (Transformation|GetVelocity _character) "0, 0, 0" (Variables|Settings-Hold|GetConsiderPlayerVelocity))) (Variables|Default|GetTarget) (Variables|Settings-Hold|GetHoldSpeedMultiplier) (Variables|Settings-Hold|GetHoldAngularReduction) (Variables|Settings-Global|GetGravity)))))

(fn ConstructionScript
  (|CallParentFunction))