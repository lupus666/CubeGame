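; Base Blueprint for telekinetic abilities, providing shared helpers to find valid targets and push them around.
; Targets are simulating static mesh actors, mostly gated by AffectPhysicsMeshes, or other actors implementing BI_Target.
; Velocity, force and impulse helpers act on mesh physics directly or route through interface messages.
; AddForceToward steers with velocity-damped, mass-independent force; AddImpulseToward cancels current motion and launches with flight-time-based gravity compensation.
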(fn ConstructionScript)

(fn IsTelekineticTarget
  (params (Target :type Actor%20Object%20Reference))
  (bind _asstatic_mesh_actor (Utilities|Casting|CastToStaticMeshActor Target)
    (:then
      (return (and (Physics|IsSimulatingPhysics (Variables|/Script/Engine.StaticMeshActor|GetStaticMeshComponent _asstatic_mesh_actor) "None") (Variables|Settings-General|GetAffectPhysicsMeshes))))
    (:CastFailed
      (return (Utilities|DoesObjectImplementInterface Target "/Game/TelekineticAbilities/Blueprints/Interfaces/BI_Target.BI_Target_C")))))

(fn FilterTargets
  (params (Targets :type Array%20of%20Actor%20Object%20References))
  (for _array_element Targets
    (bind _asstatic_mesh_actor (Utilities|Casting|CastToStaticMeshActor _array_element)
      (:then
        (if (and (Physics|IsSimulatingPhysics (Variables|/Script/Engine.StaticMeshActor|GetStaticMeshComponent _asstatic_mesh_actor) "None") (Variables|Settings-General|GetAffectPhysicsMeshes))
          (Utilities|Set|Add (LocalVariables|GettFiltered) _array_element)))
      (:CastFailed
        (if (Utilities|DoesObjectImplementInterface _array_element "/Game/TelekineticAbilities/Blueprints/Interfaces/BI_Target.BI_Target_C")
          (Utilities|Set|Add (LocalVariables|GettFiltered) _array_element)))))
  (bind _result (Utilities|Set|ToArray (LocalVariables|GettFiltered)))
  (return _result))

(fn FilterHitTargets
  (params (Targets :type Array%20of%20Hit%20Result%20Structures))
  (for _array_element Targets
    (bind _asstatic_mesh_actor (Utilities|Casting|CastToStaticMeshActor (.HitActor (Collision|BreakHitResult _array_element)))
      (:then
        (if (Physics|IsSimulatingPhysics (Variables|/Script/Engine.StaticMeshActor|GetStaticMeshComponent _asstatic_mesh_actor) "None")
          (Utilities|Set|Add (LocalVariables|GettFiltered) (.HitActor (Collision|BreakHitResult _array_element)))))
      (:CastFailed
        (if (Utilities|DoesObjectImplementInterface (.HitActor (Collision|BreakHitResult _array_element)) "/Game/TelekineticAbilities/Blueprints/Interfaces/BI_Target.BI_Target_C")
          (Utilities|Set|Add (LocalVariables|GettFiltered) (.HitActor (Collision|BreakHitResult _array_element)))))))
  (bind _result (Utilities|Set|ToArray (LocalVariables|GettFiltered)))
  (return _result))

(fn GetTargetVelocity
  (params (Target :type Actor%20Object%20Reference))
  (bind _asstatic_mesh_actor (Utilities|Casting|CastToStaticMeshActor Target)
    (:then
      (bind _returnvalue (Physics|GetPhysicsLinearVelocity (Variables|/Script/Engine.StaticMeshActor|GetStaticMeshComponent _asstatic_mesh_actor) "None"))
      (return _returnvalue (Class|PrimitiveComponent|GetPhysicsAngularVelocityinRadians (Variables|/Script/Engine.StaticMeshActor|GetStaticMeshComponent _asstatic_mesh_actor) "None")))
    (:CastFailed
      (bind (_velocity _angularvelocity) (Class|BITarget|AbilityGetVel(Message) Target))
      (return _velocity _angularvelocity))))

(fn AddImpulse
  (params (Target :type Actor%20Object%20Reference) (Impulse :type Vector) (Angular :type Vector) (IgnoreMass :type Boolean))
  (Utilities|IsValid Target
    (:Is%20Valid
      (bind _asstatic_mesh_actor (Utilities|Casting|CastToStaticMeshActor Target)
        (:then
          (Physics|AddImpulse (Variables|/Script/Engine.StaticMeshActor|GetStaticMeshComponent _asstatic_mesh_actor) Impulse "None" IgnoreMass)
          (Class|PrimitiveComponent|AddAngularImpulseinRadians (Variables|/Script/Engine.StaticMeshActor|GetStaticMeshComponent _asstatic_mesh_actor) Angular "None" IgnoreMass))
        (:CastFailed
          (Class|BITarget|AbilityImpulse(Message) Target Impulse Angular IgnoreMass))))))

(fn AddForce
  (params (Target :type Actor%20Object%20Reference) (Force :type Vector) (Torque :type Vector) (IgnoreMass :type Boolean))
  (Utilities|IsValid Target
    (:Is%20Valid
      (bind _asstatic_mesh_actor (Utilities|Casting|CastToStaticMeshActor Target)
        (:then
          (Physics|AddForce (Variables|/Script/Engine.StaticMeshActor|GetStaticMeshComponent _asstatic_mesh_actor) Force "None" IgnoreMass)
          (Class|PrimitiveComponent|AddTorqueinRadians (Variables|/Script/Engine.StaticMeshActor|GetStaticMeshComponent _asstatic_mesh_actor) Torque "None" IgnoreMass))
        (:CastFailed
          (Class|BITarget|AbilityForce(Message) Target Force Torque IgnoreMass))))))

(fn AddForceToward
  (params (Target :type Vector) (Actor :type Actor%20Object%20Reference) (Speed :type Float%20%28single-precision%29) (AngularReduction :type Float%20%28single-precision%29) (Gravity :type Float%20%28single-precision%29))
  (Utilities|IsValid Actor
    (:Is%20Valid
      (bind (_velocity _angularvelocity) (CallFunction|GetTargetVelocity Actor))
      (CallFunction|AddForce Actor (+ (* (- (- Target (Transformation|GetActorLocation Actor)) _velocity) Speed) (Math|Vector|MakeVector 0.0 0.0 Gravity)) (* _angularvelocity (* AngularReduction -1.0)) true))))

(fn AddImpulseToward
  (params (Actor :type Actor%20Object%20Reference) (Target :type Vector) (Force :type Float%20%28single-precision%29) (Gravity :type Float%20%28single-precision%29))
  (bind _output_get (LocalVariables|SetDelta (- Target (Transformation|GetActorLocation Actor))))
  (LocalVariables|SetTime (/ (Math|Vector|VectorLength _output_get) Force))
  (bind (_velocity _angularvelocity) (CallFunction|GetTargetVelocity Actor))
  (CallFunction|AddImpulse Actor (+ (* _velocity -1.0) (* (Math|Vector|Normalize _output_get) Force) (Math|Vector|MakeVector 0.0 0.0 (* (* (LocalVariables|GetTime) 0.5) Gravity))) (* _angularvelocity -1.0) true))

(fn SetDefaultFloatValue
  (params (Variable :type Float%20%28single-precision%29%20%28by%20ref%29) (Value :type Float%20%28single-precision%29))
  (if (== Variable 0.0)
    (|SetBy-RefVar Variable Value)))