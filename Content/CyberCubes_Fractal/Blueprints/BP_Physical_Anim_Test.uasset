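; Test actor that runs physical animation on a skeletal mesh with an attached electric Niagara effect.
; On BeginPlay it simulates the bodies below a configurable bone and applies physical animation drives to pull them toward the animated pose.
; Each Tick it sets the drive strength from RelaxRate and pushes two animations and their blend alpha into ABP_Physical_AnimTest.
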(event EventTick
  (params (DeltaSeconds :type Float%20%28single-precision%29))
  (Class|PhysicalAnimationComponent|SetStrengthMultiplyer (Variables|Default|GetPhysicalAnimation) (Variables|Default|GetRelaxRate))
  (bind _asabp_physical_anim_test (Utilities|Casting|CastToABP_Physical_AnimTest (Components|SkeletalMesh|GetAnimInstance (Variables|SkeletalMeshActor|GetSkeletalMeshComponent))))
  (Variables|/Game/CyberCubes_Fractal/Blueprints/ABP_Physical_AnimTest.ABP_Physical_AnimTest_C|SetAnimation%201 _asabp_physical_anim_test (Variables|Default|GetAnimation%201))
  (Variables|/Game/CyberCubes_Fractal/Blueprints/ABP_Physical_AnimTest.ABP_Physical_AnimTest_C|SetAnimation%20%202 _asabp_physical_anim_test (Variables|Default|GetAnimation%202))
  (Variables|/Game/CyberCubes_Fractal/Blueprints/ABP_Physical_AnimTest.ABP_Physical_AnimTest_C|Setanimation%20blend%20alpha _asabp_physical_anim_test (Variables|Default|GetAnimation%20Blend%20Alpha)))

(event Collision|EventActorBeginOverlap
  (params (OtherActor :type Actor%20Object%20Reference)))

(event EventBeginPlay
  (bind _skeletalmeshcomponent (Variables|SkeletalMeshActor|GetSkeletalMeshComponent))
  (bind _body_name (Variables|Default|GetBody%20Name))
  (bind _physicalanimation (Variables|Default|GetPhysicalAnimation))
  (Class|PhysicalAnimationComponent|SetSkeletalMeshComponent _physicalanimation _skeletalmeshcomponent)
  (Class|PhysicalAnimationComponent|ApplyPhysicalAnimationSettingsBelow _physicalanimation _body_name (Utilities|Struct|MakePhysicalAnimationData false 1e+03 15.0 1e+03 3e+01) false)
  (Class|SkeletalMeshComponent|SetAllBodiesBelowSimulatePhysics _skeletalmeshcomponent _body_name true false)
  ;[1 1 1] electric
  (Niagara|SpawnSystemAttached "/Game/CyberCubes_Fractal/Niagara/FXS_Electric.FXS_Electric" (Variables|SkeletalMeshActor|GetSkeletalMeshComponent) "None" "0, 0, 0" "0, 0, 0" "KeepRelativeOffset" false))

(fn ConstructionScript)