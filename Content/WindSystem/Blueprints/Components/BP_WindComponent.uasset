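; Actor component that registers its owner with a wind zone and drives movement sounds for its mesh.
; InitializeWindComponent receives the mesh and audio component, then applies damping and the sound cue.
; BeginPlay adds the owner to the first BP_WindZoneBase's affected-actor list, retrying after a delay for late actors.
; Hits play one-shot sounds above a speed threshold, while Tick feeds velocity into RollSpeed for loops, only near the camera.
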(event Custom|OnComponentHit
  (params (HitComponent :type Primitive%20Component%20Object%20Reference) (OtherActor :type Actor%20Object%20Reference) (OtherComp :type Primitive%20Component%20Object%20Reference) (NormalImpulse :type Vector) (Hit :type Hit%20Result%20Structure%20%28by%20ref%29))
  ;[1 1 1] is not using looped sound but one shot sound
  (if (not (Variables|Relevant|GetIsUsingSoundLoop))
    ;[1 1 1] plays sound on collision
    (if (> (Math|Vector|VectorLength (Transformation|GetComponentVelocity (Variables|Internal|GetMesh))) 1e+02)
      (Audio|Components|Audio|Play (Variables|Internal|GetAudioComponent) 0.0))))

(event Custom|GetWindZone
  ;[1 1 1] make sure late actors get registered
  ;[1 1 1] get  windzone
  (bind _outactors (Actor|GetAllActorsOfClass "/Game/WindSystem/Blueprints/BaseClasses/BP_WindZoneBase.BP_WindZoneBase_C"))
  (Utilities|IsValid (Utilities|Array|Get(acopy) _outactors)
    (:Is%20Valid
      (bind _output_get (Variables|Internal|SetCurrentWindzone (Utilities|Array|Get(acopy) _outactors)))
      ;[1 1 1] add actor to affected actors list
      (Utilities|Array|AddUnique (Variables|/Game/WindSystem/Blueprints/BaseClasses/BP_WindZoneBase.BP_WindZoneBase_C|GetReceivedStandardActors _output_get) (Components|GetOwner self)))))

(event EventBeginPlay
  (bind _mesh (Variables|Internal|GetMesh))
  (Utilities|IsValid _mesh
    (:Is%20Valid
      (Collision|AssignOnComponentHit _mesh (delegate Custom|OnComponentHit))
      (CallFunction|GetWindZone)
      ;[1 1 1] make sure late actors get registered
      (Utilities|Time|SetTimerbyEvent (delegate Custom|GetWindZone) 2.0))))

(event EventTick
  (params (DeltaSeconds :type Float%20%28single-precision%29))
  (bind _mesh (Variables|Internal|GetMesh))
  (bind _mesh_2 (Variables|Internal|GetMesh))
  (Utilities|IsValid _mesh_2
    (:Is%20Valid
      ;[1 1 1] increase volume of sound cue, based on velocity. only relevant for looping sounds
      (if (< (Math|Vector|VectorLength (- (Transformation|GetWorldLocation _mesh_2) (Camera|GetCameraLocation (Variables|/Script/Engine.PlayerController|GetPlayerCameraManager (Game|GetPlayerController 0))))) 1.5e+03)
        (Utilities|IsValid _mesh
          (:Is%20Valid
            (Audio|Parameter|SetFloatParameter (Variables|Internal|GetAudioComponent) "RollSpeed" (Math|Float|MapRangeClamped (Math|Vector|VectorLength (Transformation|GetComponentVelocity _mesh)) 0.0 1.5e+02 0.0 1.0) :!class /Script/Engine.AudioComponent)))))))

(fn InitializeWindComponent
  (params (Audio :type Audio%20Component%20Object%20Reference) (Mesh :type Mesh%20Component%20Object%20Reference))
  (Variables|Internal|SetAudioComponent Audio)
  (Variables|Internal|SetMesh Mesh)
  (Utilities|FlowControl|Sequence
    (:then_0
      (Class|PrimitiveComponent|SetAngularDamping (Variables|Internal|GetMesh) (Variables|Relevant|GetAngularDamping))
      (Class|PrimitiveComponent|SetLinearDamping (Variables|Internal|GetMesh) (Variables|Relevant|GetLinearDamping)))
    (:then_1
      (Audio|Components|Audio|SetSound (Variables|Internal|GetAudioComponent) (Variables|Relevant|GetSoundCue))
      (return))))