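; Electric statue prop with a bobbing center sphere that throws Niagara lightning beams toward sockets on its static mesh.
; The construction script caches socket world locations, stores the sphere's start position and sets its mesh and distortion material.
; A timeline bobs the sphere along weighted axes around that position.
; A looping 0.1-second timer re-aims the beam from the sphere to random socket points with Y/Z jitter and refreshes its two colors.
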(event Custom|Electro
  (bind _niagara (Variables|Default|GetNiagara))
  (bind _socketlocation (Variables|Default|GetSocketlocation))
  (bind _niagara_2 (Variables|Default|GetNiagara))
  (bind _jitter (Variables|Default|GetJitter))
  (bind _returnvalue (Utilities|Array|Length _socketlocation))
  (bind _returnvalue_2 (* _jitter -1.0))
  (bind _returnvalue_3 (Math|Random|RandomFloatinRange _returnvalue_2 _jitter))
  (bind _returnvalue_4 (- _returnvalue 1))
  (bind _returnvalue_5 (Math|Random|RandomIntegerinRange 0 _returnvalue_4))
  (bind _output (Utilities|Array|Get(acopy) _socketlocation _returnvalue_5))
  (bind (_x _y _z) (Class|KismetMathLibrary|BreakVector3f _output))
  (Niagara|SetNiagaraVariable(Vector3) _niagara "User.Beam Start" (Transformation|GetWorldLocation (Variables|Default|GetSphere)))
  (Niagara|SetNiagaraVariable(Vector3) _niagara "User.Beam End" (Math|Vector|MakeVector _x (+ _y _returnvalue_3) (+ _z _returnvalue_3)))
  (Niagara|SetNiagaraVariable(LinearColor) _niagara_2 "User.NiagaraParticleColor1" (Variables|Default|GetColor1))
  (Niagara|SetNiagaraVariable(LinearColor) _niagara_2 "User.NiagaraParticleColor2" (Variables|Default|GetColor2)))

(event Custom|Socket
  (for _array_element (Transformation|GetAllSocketNames (Variables|Default|GetStaticMesh))
    (Utilities|Array|Add (Variables|Default|GetSocketlocation) (Transformation|GetSocketLocation (Variables|Default|GetStaticMesh) _array_element))))

(event Custom|CustomEvent_0
  (CallFunction|Electro))

(event Custom|BobbleEvent
  (bind _inıtposition (Variables|Default|GetInıtPosition))
  (bind _boobleaxis (Variables|Default|GetBoobleAxis))
  (bind _bobble (Variables|Default|GetBobble))
  (bind (_x _y _z) (Class|KismetMathLibrary|BreakVector3f _inıtposition))
  (Components|Timeline|SetPlayRate (Variables|Default|GetTimeline_0) (Variables|Default|GetBobbleSpeed))
  (bind _newtrack_0 (Timeline|Timeline_0 Play)
    (:Update
      (Transformation|SetRelativeLocation (Variables|Default|GetSphere) (Math|Vector|MakeVector (+ _x (Math|Float|Lerp 0.0 (Math|Float|Lerp (* _bobble -1.0) _bobble _newtrack_0) (.x _boobleaxis))) (+ _y (Math|Float|Lerp 0.0 (Math|Float|Lerp (* _bobble -1.0) _bobble _newtrack_0) (.y _boobleaxis))) (+ _z (Math|Float|Lerp 0.0 (Math|Float|Lerp (* _bobble -1.0) _bobble _newtrack_0) (.z _boobleaxis)))) false false))))

(event EventBeginPlay
  (CallFunction|BobbleEvent)
  (Utilities|Time|SetTimerbyEvent (delegate Custom|CustomEvent_0) 0.1 true))

(fn ConstructionScript
  (bind _sphere (Variables|Default|GetSphere))
  (CallFunction|Socket)
  (CallFunction|Electro)
  (Variables|Default|SetInıtPosition (Variables|/Script/Engine.SceneComponent|GetRelativeLocation (Variables|Default|GetSphere)))
  (Components|StaticMesh|SetStaticMesh _sphere (Variables|Default|GetCenterMesh))
  (Rendering|Material|SetMaterial _sphere 0 "/Game/Hallway/Materials/MI_Distortion_2.MI_Distortion_2"))