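; BP_BigFan is a scene fan actor that spins its mesh continuously and plays a looping fan sound.
; BeginPlay resets the angle and starts the FanLoop cue through APCAudioComponent.
; Each Tick advances the angle by Speed scaled by delta time, wrapping it past 360 degrees.
; UpdateFanRotation combines that Y-axis rotation with the actor's rotation and sets it as the mesh's world rotation.
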(event Custom|UpdateFanRotation
  (params (Angle :type Float%20%28double-precision%29))
  ;[1 1 1] Update fan rotation
  (Transformation|SetWorldRotation (Variables|Default|GetFanMesh) (Math|Rotator|CombineRotators (Math|Vector|RotatorfromAxisandAngle (Math|Vector|MakeVector 0.0 1.0 0.0) Angle) (Transformation|GetActorRotation)) false false))

(event EventBeginPlay
  (bind _apc_audiocomponent (Variables|Default|GetAPC_AudioComponent))
  ;[1 1 1] Init
  (Variables|Default|SetCurrAngle 0.0)
  (Default|Init _apc_audiocomponent 0 0 "/Game/AdvancedPuzzleConstructor/Sounds/Cue/FanLoop_Cue.FanLoop_Cue" 1.0)
  (Default|StarttoLoop _apc_audiocomponent))

(event EventTick
  (params (DeltaSeconds :type Float%20%28single-precision%29))
  ;[1 1 1] Rotate fan
  (bind _output_get (Variables|Default|SetDeltaTime DeltaSeconds))
  (bind _output_get_2 (Variables|Default|SetCurrAngle (+ (Variables|Default|GetCurrAngle) (* _output_get (Variables|Default|GetSpeed)))))
  (if (> _output_get_2 3.6e+02)
    (Variables|Default|SetCurrAngle (- (+ (Variables|Default|GetCurrAngle) (* _output_get (Variables|Default|GetSpeed))) 3.6e+02)))
  (CallFunction|UpdateFanRotation (Variables|Default|GetCurrAngle)))

(fn ConstructionScript)