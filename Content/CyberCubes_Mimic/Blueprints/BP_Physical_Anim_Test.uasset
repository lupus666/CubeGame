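; Test actor that drives a skeletal mesh with physical animation and attaches an electric effect to it.
; On BeginPlay it applies strong orientation and position drives to bodies below a configurable bone, excluding that bone, and sets those bodies simulating.
; Tick continually feeds RelaxRate into the physical animation strength multiplier, controlling how closely the simulated bodies follow the animation.
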(event EventTick
  (params (DeltaSeconds :type Float%20%28single-precision%29))
  (Class|PhysicalAnimationComponent|SetStrengthMultiplyer (Variables|Default|GetPhysicalAnimation) (Variables|Default|GetRelaxRate)))

(event Collision|EventActorBeginOverlap
  (params (OtherActor :type Actor%20Object%20Reference)))

(event EventBeginPlay
  (bind _skeletalmeshcomponent (Variables|SkeletalMeshActor|GetSkeletalMeshComponent))
  (bind _body_name (Variables|Default|GetBody%20Name))
  (bind _physicalanimation (Variables|Default|GetPhysicalAnimation))
  (Class|PhysicalAnimationComponent|SetSkeletalMeshComponent _physicalanimation _skeletalmeshcomponent)
  (Class|PhysicalAnimationComponent|ApplyPhysicalAnimationSettingsBelow _physicalanimation _body_name (Utilities|Struct|MakePhysicalAnimationData false 1e+03 15.0 1e+03 3e+01) false)
  (Class|SkeletalMeshComponent|SetAllBodiesBelowSimulatePhysics _skeletalmeshcomponent _body_name true false)
  ;[1 1 1] electric
  (Niagara|SpawnSystemAttached "/Game/CyberCubes_Mimic/Niagara/FXS_Electric.FXS_Electric" (Variables|SkeletalMeshActor|GetSkeletalMeshComponent) "None" "0, 0, 0" "0, 0, 0" "KeepRelativeOffset" false))

(fn ConstructionScript)