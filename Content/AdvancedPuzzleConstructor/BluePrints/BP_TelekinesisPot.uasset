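; BP_TelekinesisPot is a puzzle pot that reports itself as telekinesis-compatible and grabbable, but not transportable or teleportable.
; On deploy start, it disables gravity and plays a timeline that nudges the mesh toward the weapon target with scaled roll and pitch distortion.
; Stopping deploy restores the configured gravity and halts the timeline.
; Interface functions supply its transform and mostly fixed answers to other puzzle systems, while usability depends on custom state.
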(event EventBeginPlay
  ;[1 0.8363 0.0916] Init
  (|CallParentFunction)
  (Components|Timeline|SetPlayRate (Variables|Default|GetDeploy) (Variables|Default|GetDistortionPlayRate)))

(event Collision|EventActorBeginOverlap
  (params (OtherActor :type Actor%20Object%20Reference))
  (|CallParentFunction OtherActor) ; This node is disabled and will not be called.\nDrag off pins to build functionality.
)

(event EventTick
  (params (DeltaSeconds :type Float%20%28single-precision%29))
  (|CallParentFunction DeltaSeconds))

(event EventStartDeploy
  (bind _deploydistortionscale (Variables|Default|GetDeployDistortionScale))
  (bind _staticmesh (Variables|Default|GetStaticMesh))
  ;[1 1 1] Deploy Stage. You can implement your deploy animation
  (Variables|Default|SetStartObjectLocation (Transformation|GetWorldLocation _staticmesh))
  (Variables|Default|SetStartObjectRotation (Transformation|GetWorldRotation _staticmesh))
  (Physics|SetEnableGravity (Variables|Default|GetStaticMesh) false)
  (bind _deployanim (Timeline|Deploy PlayFromStart)
    (:Update
      (Transformation|SetWorldLocationAndRotation (Variables|Default|GetStaticMesh) (+ (* (Math|Vector|Normalize (- (Variables|Default|GetWeaponTargetLocation) (Variables|Default|GetStartObjectLocation))) (* (.X (Math|Vector|BreakVector _deployanim)) (.x _deploydistortionscale))) (Variables|Default|GetStartObjectLocation)) (Math|Rotator|CombineRotators (Math|Rotator|MakeRotator (* (.Y (Math|Vector|BreakVector _deployanim)) (.y _deploydistortionscale)) (* (.Z (Math|Vector|BreakVector _deployanim)) (.z _deploydistortionscale)) 0.0) (Variables|Default|GetStartObjectRotation)) false false))))

(event EventStopDeploy
  (bind _deploydistortionscale (Variables|Default|GetDeployDistortionScale))
  ;[1 1 1] Deploy Stage. You can implement your deploy animation
  (Physics|SetEnableGravity (Variables|Default|GetStaticMesh) (Variables|Default|GetEnableGravity))
  (bind _deployanim (Timeline|Deploy Stop)
    (:Update
      (Transformation|SetWorldLocationAndRotation (Variables|Default|GetStaticMesh) (+ (* (Math|Vector|Normalize (- (Variables|Default|GetWeaponTargetLocation) (Variables|Default|GetStartObjectLocation))) (* (.X (Math|Vector|BreakVector _deployanim)) (.x _deploydistortionscale))) (Variables|Default|GetStartObjectLocation)) (Math|Rotator|CombineRotators (Math|Rotator|MakeRotator (* (.Y (Math|Vector|BreakVector _deployanim)) (.y _deploydistortionscale)) (* (.Z (Math|Vector|BreakVector _deployanim)) (.z _deploydistortionscale)) 0.0) (Variables|Default|GetStartObjectRotation)) false false))))

(fn ConstructionScript
  (|CallParentFunction))

(fn IsTelekinesisCompatibleBPI
  ;[1 1 1] Return Telekekinesis type
  (return true))

(fn GetPushBoxDataBPI
  (return 0.0 "" ""))

(fn IsObjectTransportableBPI
  (return false))

(fn IsObjectTeleportableBPI
  (return false))

(fn GetVoltageCapacityBPI
  (return 0.0 0.0))

(fn GetBoxTransformBPI
  (return (Transformation|GetWorldTransform (Variables|Default|GetStaticMesh))))

(fn IsAttachedtoConveyorBPI
  (return false))

(fn GetBoxColorandStateBPI
  (return "NewEnumerator1" false false false))

(fn GetObjectTypeBPI
  ;[1 1 1] Return that object can be Grabbed
  (return "NewEnumerator7"))

(fn ObjectCanbeUsed
  ;[1 1 1] Is custom state?
  (return (not (Variables|Default|GetCustomState))))

(fn GetTargetTransform
  (return ""))