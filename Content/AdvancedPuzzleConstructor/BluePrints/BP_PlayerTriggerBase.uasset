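; Base trigger volume for the Advanced Puzzle Constructor that detects the player entering and leaving its OverlapArea.
; Overlaps count only while Enabled, toggled by Activate/Deactivate interface events, and only for actors with the player tag.
; It passes the actor and its ACP controller to empty PlayerInTrigger and PlayerOutFromTrigger events for children to override.
; With UseOnce, the first exit marks it used; other interface functions return defaults.
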(event OnComponentBeginOverlap(OverlapArea)
  (params (OverlappedComponent :type Primitive%20Component%20Object%20Reference) (OtherActor :type Actor%20Object%20Reference) (OtherComp :type Primitive%20Component%20Object%20Reference) (OtherBodyIndex :type Integer) (bFromSweep :type Boolean) (SweepResult :type Hit%20Result%20Structure%20%28by%20ref%29))
  ;[1 1 1] Begin overlap
  (if (Variables|PlayerTrigger|GetEnabled)
    (if (not (Variables|Default|GetIsUsed))
      (if (Actor|ActorHasTag OtherActor (CallFunction|LIBGetPlayerTag))
        (bind _apccontroller (CallFunction|LIBGetACPController OtherActor))
        (CallFunction|PlayerinTrigger OtherActor _apccontroller)))))

(event OnComponentEndOverlap(OverlapArea)
  (params (OverlappedComponent :type Primitive%20Component%20Object%20Reference) (OtherActor :type Actor%20Object%20Reference) (OtherComp :type Primitive%20Component%20Object%20Reference) (OtherBodyIndex :type Integer))
  ;[1 1 1] End overlap
  (if (Variables|PlayerTrigger|GetEnabled)
    (if (not (Variables|Default|GetIsUsed))
      (if (Actor|ActorHasTag OtherActor (CallFunction|LIBGetPlayerTag))
        (bind _apccontroller (CallFunction|LIBGetACPController OtherActor))
        (CallFunction|PlayerOutfromTrigger OtherActor _apccontroller)
        (if (Variables|PlayerTrigger|GetUseOnce)
          (Variables|Default|SetIsUsed true))))))

(event Custom|PlayerInTrigger
  (params (PlayerActor :type Actor%20Object%20Reference) (APC_Controller :type Actor%20Component%20Object%20Reference))
  ;[0.02728 1 0.2986] Called when player is inside of trigger or leave trigger volume
)

(event Custom|PlayerOutFromTrigger
  (params (PlayerActor :type Actor%20Object%20Reference) (APC_Controller :type Actor%20Component%20Object%20Reference))
  ;[0.02728 1 0.2986] Called when player is inside of trigger or leave trigger volume
)

(event EventBeginPlay
  ;[1 0.7655 0.1745] Begin Play init
  (Variables|Default|SetIsUsed false))

(event EventActivateBPI
  ;[1 1 1] Activate / deactvate events
  (Variables|PlayerTrigger|SetEnabled true))

(event EventDeactivateBPI
  ;[1 1 1] Activate / deactvate events
  (Variables|PlayerTrigger|SetEnabled false))

(fn ConstructionScript)

(fn AnimGetForwardAxisBPI
  (return 0.0))

(fn AnimIsonLadderBPI
  (return false))

(fn AnimIsPushingBoxBPI
  (return false 0.0 "" ""))

(fn CanbeUsedBPI
  (return false))

(fn GetCapsuleHalfHeightBPI
  (return 0.0))

(fn GetCapsuleRadiusBPI
  (return 0.0))

(fn GetCapsuleTransformBPI
  (return ""))

(fn GetCharacterControllerBPI
  (return 0))

(fn GetCharacterControlRotationBPI
  (return "0, 0, 0"))

(fn HasOverlappedObjectBPI
  (return false))

(fn IsActorActivatedBPI
  (return false))