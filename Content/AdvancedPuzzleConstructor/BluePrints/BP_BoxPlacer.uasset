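; Puzzle socket that captures boxes entering either detect volume and stacks them at a target arrow until BoxCount is reached.
; Captured boxes are detached from the player, stripped of physics and queued, then Tick lerps each horizontally and drops it into its slot via BPI interface messages.
; Completing the stack deactivates the linked player blockers and stops further capture.
; The construction script fits the block area and detect volume heights to BoxCount.
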(event OnComponentBeginOverlap(BlockArea)
  (params (OverlappedComponent :type Primitive%20Component%20Object%20Reference) (OtherActor :type Actor%20Object%20Reference) (OtherComp :type Primitive%20Component%20Object%20Reference) (OtherBodyIndex :type Integer) (bFromSweep :type Boolean) (SweepResult :type Hit%20Result%20Structure%20%28by%20ref%29)))

(event OnComponentBeginOverlap(DetectVolume1)
  (params (OverlappedComponent :type Primitive%20Component%20Object%20Reference) (OtherActor :type Actor%20Object%20Reference) (OtherComp :type Primitive%20Component%20Object%20Reference) (OtherBodyIndex :type Integer) (bFromSweep :type Boolean) (SweepResult :type Hit%20Result%20Structure%20%28by%20ref%29))
  ;[1 1 1] Check if there is any boxes are ovelapping
  (Variables|Default|SetOverlappedActor OtherActor)
  (if (Variables|Default|GetEnabled)
    (if (not (Variables|Default|GetIsBoxPlaced))
      (if (Utilities|DoesObjectImplementInterface (Variables|Default|GetOverlappedActor) "/Game/AdvancedPuzzleConstructor/BluePrints/Core/BPI_ObjectControls.BPI_ObjectControls_C")
        (bind _objecttype (Class|BPIObjectControls|GetObjectTypeBPI(Message) (Variables|Default|GetOverlappedActor)))
        (if (Utilities|Enum|Equal(Enum) _objecttype "NewEnumerator0")
          (bind (_boxtype _inair _incustomstate _isattachedtoplayer) (Class|BPIObjectControls|GetBoxColorandStateBPI(Message) (Variables|Default|GetOverlappedActor)))
          (if (not _incustomstate)
            (if _isattachedtoplayer
              (Class|BPIObjectControls|DetachfromPlayerBPI(Message) (Variables|Default|GetOverlappedActor)))
            (Class|BPIObjectControls|SetCustomStateBPI(Message) (Variables|Default|GetOverlappedActor) true)
            (Class|BPIObjectControls|EnableMeshPhysicBPI(Message) (Variables|Default|GetOverlappedActor) false)
            (Class|BPIObjectControls|EnableMeshGravityBPI(Message) (Variables|Default|GetOverlappedActor) false)
            (bind _boxtransform (Class|BPIObjectControls|GetBoxTransformBPI(Message) (Variables|Default|GetOverlappedActor)))
            (Class|BPIObjectControls|HideWidgetsBPI(Message) (Variables|Default|GetOverlappedActor) true)
            (Utilities|Array|Add (Variables|Default|GetProcessingBoxes) (Utilities|Struct|MakeF_PlayerBlocker (Variables|Default|GetOverlappedActor) 0.0 false (.location _boxtransform) (+ (Transformation|GetWorldLocation (Variables|Default|GetTargetArrow)) (Math|Vector|MakeVector 0.0 0.0 (* (Variables|Default|GetPassedBoxesCount) (* (Variables|Default|GetBoxHalfSize) 2.0))))))
            (Math|Integer|IncrementInt (Variables|Default|GetPassedBoxesCount))))))))

(event OnComponentBeginOverlap(DetectVolume2)
  (params (OverlappedComponent :type Primitive%20Component%20Object%20Reference) (OtherActor :type Actor%20Object%20Reference) (OtherComp :type Primitive%20Component%20Object%20Reference) (OtherBodyIndex :type Integer) (bFromSweep :type Boolean) (SweepResult :type Hit%20Result%20Structure%20%28by%20ref%29))
  ;[1 1 1] Check if there is any boxes are ovelapping
  (Variables|Default|SetOverlappedActor OtherActor)
  (if (Variables|Default|GetEnabled)
    (if (not (Variables|Default|GetIsBoxPlaced))
      (if (Utilities|DoesObjectImplementInterface (Variables|Default|GetOverlappedActor) "/Game/AdvancedPuzzleConstructor/BluePrints/Core/BPI_ObjectControls.BPI_ObjectControls_C")
        (bind _objecttype (Class|BPIObjectControls|GetObjectTypeBPI(Message) (Variables|Default|GetOverlappedActor)))
        (if (Utilities|Enum|Equal(Enum) _objecttype "NewEnumerator0")
          (bind (_boxtype _inair _incustomstate _isattachedtoplayer) (Class|BPIObjectControls|GetBoxColorandStateBPI(Message) (Variables|Default|GetOverlappedActor)))
          (if (not _incustomstate)
            (if _isattachedtoplayer
              (Class|BPIObjectControls|DetachfromPlayerBPI(Message) (Variables|Default|GetOverlappedActor)))
            (Class|BPIObjectControls|SetCustomStateBPI(Message) (Variables|Default|GetOverlappedActor) true)
            (Class|BPIObjectControls|EnableMeshPhysicBPI(Message) (Variables|Default|GetOverlappedActor) false)
            (Class|BPIObjectControls|EnableMeshGravityBPI(Message) (Variables|Default|GetOverlappedActor) false)
            (bind _boxtransform (Class|BPIObjectControls|GetBoxTransformBPI(Message) (Variables|Default|GetOverlappedActor)))
            (Class|BPIObjectControls|HideWidgetsBPI(Message) (Variables|Default|GetOverlappedActor) true)
            (Utilities|Array|Add (Variables|Default|GetProcessingBoxes) (Utilities|Struct|MakeF_PlayerBlocker (Variables|Default|GetOverlappedActor) 0.0 false (.location _boxtransform) (+ (Transformation|GetWorldLocation (Variables|Default|GetTargetArrow)) (Math|Vector|MakeVector 0.0 0.0 (* (Variables|Default|GetPassedBoxesCount) (* (Variables|Default|GetBoxHalfSize) 2.0))))))
            (Math|Integer|IncrementInt (Variables|Default|GetPassedBoxesCount))))))))

(event Custom|EnablePlayerBlockers
  (params (EnableBlocker :type Boolean))
  ;[1 1 1] Deactivate Player blocker specified in the PlayerBlockers array
  (for _array_element (Variables|BoxPlacer|GetPlayerBlocker)
    (if (Utilities|DoesObjectImplementInterface _array_element "/Game/AdvancedPuzzleConstructor/BluePrints/Core/BPI_Actor_Action.BPI_Actor_Action_C")
      (if EnableBlocker
        (Class|BPIActorAction|ActivateBPI(Message) _array_element)
        (else
          (Class|BPIActorAction|DeactivateBPI(Message) _array_element))))))

(event EventBeginPlay
  ;[1 0.7655 0.1745] Begin Play init
  (Variables|Default|SetIsBoxPlaced false)
  (Variables|Default|SetPassedBoxesCount 0)
  (Variables|Default|SetEnabled true)
  (Variables|Default|SetBoxHalfSize 1e+02))

(event EventTick
  (params (DeltaSeconds :type Float%20%28single-precision%29))
  ;[1 1 1] Process movement for boxes from the list
  (if (> (Utilities|Array|Length (Variables|Default|GetProcessingBoxes)) 0)
    (CallFunction|ProcessBoxes DeltaSeconds)))

(fn ConstructionScript
  (bind _blockarea (Variables|Default|GetBlockArea))
  (bind _detectvolume1 (Variables|Default|GetDetectVolume1))
  (bind _detectvolume2 (Variables|Default|GetDetectVolume2))
  (bind _boxcount (Variables|BoxPlacer|GetBoxCount))
  (bind _boxhalfsize (Variables|Default|GetBoxHalfSize))
  (bind _returnvalue (- _boxcount 1))
  (bind _returnvalue_2 (* _boxhalfsize 2.0))
  (bind _returnvalue_3 (* _returnvalue _returnvalue_2))
  (bind _returnvalue_4 (* _returnvalue _boxhalfsize))
  (bind _returnvalue_5 (+ _returnvalue_4 _boxhalfsize))
  ;[1 1 1] Adjust block area based on Box count
  (Components|Box|SetBoxExtent _blockarea (Math|Vector|MakeVector 102.0 102.0 _returnvalue_5) true)
  (Transformation|SetRelativeLocation _blockarea (Math|Vector|MakeVector 0.0 0.0 (- _returnvalue_5 _boxhalfsize)) false true)
  (Transformation|SetRelativeLocation _detectvolume1 (+ (Variables|/Script/Engine.SceneComponent|GetRelativeLocation _detectvolume1) (Math|Vector|MakeVector 0.0 0.0 _returnvalue_3)) false false)
  (Transformation|SetRelativeLocation _detectvolume2 (+ (Variables|/Script/Engine.SceneComponent|GetRelativeLocation _detectvolume2) (Math|Vector|MakeVector 0.0 0.0 _returnvalue_3)) false false))

(fn ProcessBoxes
  (params (DeltaTime :type Float%20%28single-precision%29))
  (bind _processingboxes (Variables|Default|GetProcessingBoxes))
  ;[1 1 1] Move Boxes within BoxPlacer to target locations
  (LocalVariables|SetDT DeltaTime)
  (for (_array_element _array_index) _processingboxes
    (LocalVariables|SetIndex _array_index)
    (bind _output_get (LocalVariables|SetNewLocalVar_0 _array_element))
    (LocalVariables|SetActor (.actor _output_get))
    (LocalVariables|SetCounter (Math|Float|Clamp(Float) (+ (.counter _output_get) (* (LocalVariables|GetDT) (Variables|BoxPlacer|GetSpeed)))))
    (LocalVariables|SetDrop (.dropdown _output_get))
    (LocalVariables|SetStartLoc (.startlocation _output_get))
    (LocalVariables|SetDestLoc (.targetlocation _output_get))
    (if (LocalVariables|GetDrop)
      ;;[1 1 1] Vertical transition
      (Class|BPIObjectControls|SetBoxLocationBPI(Message) (LocalVariables|GetActor) (Math|Vector|Lerp(Vector) (Math|Vector|MakeVector (.X (Math|Vector|BreakVector (LocalVariables|GetDestLoc))) (.Y (Math|Vector|BreakVector (LocalVariables|GetDestLoc))) (.Z (Math|Vector|BreakVector (LocalVariables|GetStartLoc)))) (Math|Vector|MakeVector (.X (Math|Vector|BreakVector (LocalVariables|GetDestLoc))) (.Y (Math|Vector|BreakVector (LocalVariables|GetDestLoc))) (.Z (Math|Vector|BreakVector (LocalVariables|GetDestLoc)))) (LocalVariables|GetCounter)))
      (Class|BPIObjectControls|UpdateBoxActorLocationBPI(Message) (LocalVariables|GetActor))
      (if (and (>= (LocalVariables|GetCounter) 1.0) (LocalVariables|GetDrop))
        (Class|BPIObjectControls|SetBoxCollisionBPI(Message) (LocalVariables|GetActor) false)
        (Utilities|Array|RemoveIndex _processingboxes (LocalVariables|GetIndex))
        (if (>= (Variables|Default|GetPassedBoxesCount) (Variables|BoxPlacer|GetBoxCount))
          (CallFunction|EnablePlayerBlockers false)
          (Variables|Default|SetIsBoxPlaced true))
        (else
          (Utilities|Array|SetArrayElem _processingboxes (LocalVariables|GetIndex) (Utilities|Struct|MakeF_PlayerBlocker (LocalVariables|GetActor) (LocalVariables|GetCounter) (LocalVariables|GetDrop) (LocalVariables|GetStartLoc) (LocalVariables|GetDestLoc)) :!label _label)))
      (else
        ;;[1 1 1] Horizontal transition
        (Class|BPIObjectControls|SetBoxLocationBPI(Message) (LocalVariables|GetActor) (Math|Vector|Lerp(Vector) (LocalVariables|GetStartLoc) (Math|Vector|MakeVector (.X (Math|Vector|BreakVector (LocalVariables|GetDestLoc))) (.Y (Math|Vector|BreakVector (LocalVariables|GetDestLoc))) (.Z (Math|Vector|BreakVector (LocalVariables|GetStartLoc)))) (LocalVariables|GetCounter)))
        (Class|BPIObjectControls|UpdateBoxActorLocationBPI(Message) (LocalVariables|GetActor))
        (if (>= (LocalVariables|GetCounter) 1.0)
          (LocalVariables|SetCounter 0.0)
          (LocalVariables|SetDrop true)
          (Class|BPIObjectControls|StartTransitionRotationBPI(Message) (LocalVariables|GetActor) true false)
          (goto _label)
          (else
            (goto _label)))))))