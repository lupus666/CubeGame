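; BP_VoltageIndicator is a puzzle-constructor indicator that displays a voltage level through a dynamic material on its mesh.
; BeginPlay creates the M_VoltageIndicator instance, sets its particle width and height, and doubles the mesh's bounds scale.
; Interface-style events receive voltage, driving emissive power from the clamped ratio to maximum, and show or hide the mesh.
; Every voltage update applies the discharged color and full flicker, whatever the level.
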(event EventBeginPlay
  ;[1 0.7655 0.1745] Begin Play init
  (Rendering|SetBoundsScale (Variables|Default|GetIndicatorMesh) 2.0)
  (bind _returnvalue (Rendering|Material|CreateDynamicMaterialInstance (Variables|Default|GetIndicatorMesh) 0 "/Game/AdvancedPuzzleConstructor/Materials/M_VoltageIndicator.M_VoltageIndicator" "None" :!class /Script/Engine.PrimitiveComponent))
  (bind _output_get (Variables|Default|SetBlinkerMaterial _returnvalue))
  (Rendering|Material|SetScalarParameterValue _output_get "ParticleWidth" (* (Variables|Indicator|GetWIdth) -1.0) :!class /Script/Engine.MaterialInstanceDynamic)
  (Rendering|Material|SetScalarParameterValue _output_get "ParticleHeight" (Variables|Indicator|GetHeight) :!class /Script/Engine.MaterialInstanceDynamic))

(event EventSetVoltageBPI
  (params (Voltage :type Float%20%28single-precision%29) (MaxVoltage :type Float%20%28single-precision%29))
  (bind _blinkermaterial (Variables|Default|GetBlinkerMaterial))
  ;[1 1 1] Set voltage and pass value to the material
  (Variables|Default|SetTempColor (Variables|Indicator|GetDischargedColor))
  (Variables|Default|SetFlicker 1.0)
  (Rendering|Material|SetVectorParameterValue _blinkermaterial "Color" (Variables|Default|GetTempColor) :!class /Script/Engine.MaterialInstanceDynamic)
  (Rendering|Material|SetScalarParameterValue _blinkermaterial "Flicker" (Variables|Default|GetFlicker) :!class /Script/Engine.MaterialInstanceDynamic)
  (Rendering|Material|SetScalarParameterValue _blinkermaterial "EmessivePower" (Math|Float|Clamp(Float) (/ Voltage (+ MaxVoltage 1.0))) :!class /Script/Engine.MaterialInstanceDynamic))

(event EventHideIndicatorBPI
  (params (Show :type Boolean))
  (bind _indicatormesh (Variables|Default|GetIndicatorMesh))
  ;[1 1 1] Hide / Show indicator mesh
  (if Show
    (Development|SetHiddeninGame _indicatormesh false false)
    (Transformation|SetWorldScale3D _indicatormesh "1.000000,1.000000,1.000000")
    (Rendering|SetVisibility _indicatormesh true false)
    (else
      (Development|SetHiddeninGame _indicatormesh true false)
      (Rendering|SetVisibility _indicatormesh false false))))

(fn ConstructionScript)