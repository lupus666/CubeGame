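; Base physics object for the telekinesis gun, exposing grab, pickup, deploy and physics state through interface events and getters.
; BeginPlay configures the mesh's physics; objects without gravity can get a starting impulse and receive extra impulses on hits.
; Tick counts down a timed deploy with overridable StartDeploy/StopDeploy hooks, otherwise rotating a grabbed mesh by the pivot offset captured at grab.
; Grab and target locations are only stored here.
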(event OnComponentHit(StaticMesh)
  (params (HitComponent :type Primitive%20Component%20Object%20Reference) (OtherActor :type Actor%20Object%20Reference) (OtherComp :type Primitive%20Component%20Object%20Reference) (NormalImpulse :type Vector :default "0, 0, 0") (Hit :type Hit%20Result%20Structure%20%28by%20ref%29))
  ;[1 1 1] Add impulse to the object if Hit detected
  (if (Math|Boolean|ANDBoolean (not (Variables|TelekinesisObject|GetEnableGravity)) (not (Variables|Default|GetGrabbed)) (not (Variables|Default|GetCustomState)))
    (Physics|AddImpulse (Variables|Default|GetStaticMesh) (* (.normal Hit) (Math|Vector|VectorLength (Transformation|GetVelocity OtherActor))) "None" true)))

(event Custom|StartDeploy
  ;[0.2883 1 0.212] Helper  internal events. You can override event for your own implementation
)

(event Custom|StopDeploy
  ;[0.2883 1 0.212] Helper  internal events. You can override event for your own implementation
)

(event EventBeginPlay
  (bind _staticmesh (Variables|Default|GetStaticMesh))
  (bind _staticmesh_2 (Variables|Default|GetStaticMesh))
  (bind _startimpulsedirection (Variables|Default|GetStartImpulseDirection))
  (bind _startimpulsepower (Variables|TelekinesisObject|GetStartImpulsePower))
  (bind _returnvalue (Math|Vector|GetForwardVector _startimpulsedirection))
  (bind _returnvalue_2 (* _returnvalue _startimpulsepower))
  ;[0.9941 1 0.1976] Init
  (Variables|Default|SetDoDeploy false)
  (Variables|Default|SetIsDeployed false)
  (Variables|Default|SetInPickupArea false)
  (Physics|SetEnableGravity _staticmesh (Variables|TelekinesisObject|GetEnableGravity))
  (Physics|SetSimulatePhysics _staticmesh (Variables|TelekinesisObject|GetSimulatePhysicsOnStart))
  (Class|PrimitiveComponent|SetAngularDamping _staticmesh (Variables|TelekinesisObject|GetAngularDamping))
  (Class|PrimitiveComponent|SetMassOverrideinKg _staticmesh "None" (Variables|TelekinesisObject|GetMassInKg) true)
  (if (Math|Boolean|ANDBoolean (not (Variables|TelekinesisObject|GetEnableGravity)) (> (Variables|TelekinesisObject|GetStartImpulsePower) 0.0) (Variables|TelekinesisObject|GetSimulatePhysicsOnStart))
    (Physics|AddImpulse _staticmesh_2 _returnvalue_2 "None" true)
    (Class|PrimitiveComponent|AddAngularImpulseinDegrees _staticmesh_2 _returnvalue_2 "None" true)))

(event Collision|EventActorBeginOverlap
  (params (OtherActor :type Actor%20Object%20Reference)))

(event EventEnableMeshPhysicBPI
  (params (EnablePhysic :type Boolean))
  ;[0.07462 0.519 1] Interface events
  (Physics|SetSimulatePhysics (Variables|Default|GetStaticMesh) EnablePhysic))

(event EventEnableMeshGravityBPI
  (params (Gravity :type Boolean))
  ;[0.07462 0.519 1] Interface events
  (Physics|SetEnableGravity (Variables|Default|GetStaticMesh) Gravity)
  (Variables|TelekinesisObject|SetEnableGravity Gravity))

(event EventSetCustomStateBPI
  (params (CustomState :type Boolean))
  ;[0.07462 0.519 1] Interface events
  (Variables|Default|SetCustomState CustomState))

(event EventSetAngularDampingBPI
  (params (AngularDamping :type Float%20%28single-precision%29))
  ;[0.07462 0.519 1] Interface events
  (Class|PrimitiveComponent|SetAngularDamping (Variables|Default|GetStaticMesh) AngularDamping))

(event EventTick
  (params (DeltaSeconds :type Float%20%28single-precision%29))
  ;[1 1 1] Rotation object within grab direction
  (if (Variables|Default|GetDoDeploy)
    (bind _output_get (Variables|Default|SetCurrDeployTime (Math|Float|Clamp(Float) (- (Variables|Default|GetCurrDeployTime) DeltaSeconds) 0.0 (Variables|TelekinesisObject|GetDeployTime))))
    (if (<= _output_get 0.0)
      (Variables|Default|SetIsDeployed true)
      ;[1 1 1] Start / Stop deploy interface event
      (CallFunction|StopDeploy)
      (Variables|Default|SetDoDeploy false))
    (elif (Variables|Default|GetGrabbed)
      (Transformation|SetWorldRotation (Variables|Default|GetStaticMesh) (Math|Transform|TransformRotation (Math|Transform|MakeTransform "0, 0, 0" (Variables|Default|GetGrabRotation) "1,1,1") (Variables|Default|GetGrabPivotRotation)) false false))))

(event EventStartStopDeployBPI
  (params (Start :type Boolean))
  ;[1 1 1] Start / Stop deploy interface event
  (if Start
    (if (not (Variables|Default|GetIsDeployed))
      (Variables|Default|SetCurrDeployTime (Variables|TelekinesisObject|GetDeployTime))
      (CallFunction|StartDeploy)
      (Variables|Default|SetDoDeploy true))
    (else
      (CallFunction|StopDeploy)
      (Variables|Default|SetDoDeploy false))))

(event EventSetTargetLocationBPI
  (params (Location :type Vector :default "0, 0, 0"))
  ;[0.07462 0.519 1] Interface events
  (Variables|Default|SetWeaponTargetLocation Location))

(event EventSetBoxRotationBPI
  (params (Rotation :type Rotator :default "0, 0, 0"))
  ;[0.07462 0.519 1] Interface events
  (Variables|Default|SetGrabRotation Rotation))

(event EventSetObjectGrabbedBPI
  (params (Grabbed :type Boolean))
  ;[1 1 1] Set Object grabbed
  (if Grabbed
    (Variables|Default|SetGrabPivotRotation (Math|Transform|InverseTransformRotation (Math|Transform|MakeTransform "0, 0, 0" (Transformation|GetWorldRotation (Variables|Default|GetGrabPivot)) "1,1,1") (Transformation|GetWorldRotation (Variables|Default|GetStaticMesh))))
    (Variables|Default|SetGrabbed true)
    (Transformation|SetActorTransform (Transformation|GetWorldTransform (Variables|Default|GetStaticMesh)))
    (else
      (Variables|Default|SetGrabbed false))))

(event EventSetBoxLocationBPI
  (params (Location :type Vector :default "0, 0, 0"))
  ;[0.07462 0.519 1] Interface events
  (Variables|Default|SetGrabLocation Location))

(event EventSetObjectinPickupAreaBPI
  (params (InPickupArea :type Boolean))
  ;[0.07462 0.519 1] Interface events
  (Variables|Default|SetInPickupArea InPickupArea))

(event EventSetMeshTransformBPI
  (params (Transform :type Transform))
  ;[0.07462 0.519 1] Interface events
  (Transformation|SetWorldTransform (Variables|Default|GetStaticMesh) Transform false false))

(fn ConstructionScript
  (Transformation|SetWorldScale3D (Variables|Default|GetGrabPivot) "1.000000,1.000000,1.000000"))

(fn GetAngularDampingBPI
  (return (Variables|TelekinesisObject|GetAngularDamping)))

(fn GetBoxColorandStateBPI
  (return "NewEnumerator1" false false false))

(fn GetBoxTransformBPI
  (return (Transformation|GetWorldTransform (Variables|Default|GetStaticMesh))))

(fn GetDeployTimeBPI
  (return (Math|Float|SelectFloat 0.0 (Math|Float|SelectFloat (Variables|Default|GetCurrDeployTime) (Variables|TelekinesisObject|GetDeployTime) (Variables|Default|GetDoDeploy)) (Variables|Default|GetIsDeployed))))

(fn GetGrabbingDataBPI
  (return "0, 0, 0" (Variables|Default|GetGrabSpeed) (Variables|TelekinesisObject|GetThrowPower) (Variables|TelekinesisObject|GetEnableGravityAfterThrow)))

(fn GetObjectAxisBPI
  (return (Math|Vector|GetForwardVector (Variables|Default|GetRight)) (Math|Vector|GetForwardVector (Variables|Default|GetForward)) (Math|Vector|GetForwardVector (Variables|Default|GetUp))))

(fn GetObjectTypeBPI
  (return "NewEnumerator1"))

(fn GetPushBoxDataBPI
  (return 0.0 "" ""))

(fn GetTargetTransform
  (return ""))

(fn GetVoltageCapacityBPI
  (return 0.0 0.0))

(fn IsAttachedtoConveyorBPI
  (return false))

(fn IsDeploymentinProgressBPI
  (return (Variables|Default|GetDoDeploy)))

(fn IsObjectGrabbedBPI
  (return (Variables|Default|GetGrabbed)))

(fn IsObjectinPickupAreaBPI
  (return (Variables|Default|GetInPickupArea)))

(fn IsObjectTeleportableBPI
  (return false))

(fn IsObjectTransportableBPI
  (return false))

(fn IsTelekinesisCompatibleBPI
  ;[1 1 1] Return True. Object is compatible with Telekinesis gun
  (return true))

(fn IsTelekinesisPickupableBPI
  (return (Variables|TelekinesisObject|GetPickupable)))

(fn ObjectCanbeUsed
  (return (not (Variables|Default|GetCustomState))))