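; Telekinesis-compatible, remote-controlled puzzle dial that rotates through eight 45-degree positions to trigger actions on target actors.
; Each button press plays a timeline-driven turn with looping audio, ignoring presses mid-turn.
; Landing on UnlockPosition runs each target's BoxYep action, and the next move off it runs BoxNop once.
; The construction script orients the dial and unlock marker, while spotting fades the glow through two dynamic materials.
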(event EventBeginPlay
  ;[0.9004 1 0.2708] Init
  (bind _returnvalue (Rendering|Material|CreateDynamicMaterialInstance (Variables|Default|GetBase) 0 0 "None" :!class /Script/Engine.PrimitiveComponent))
  (Variables|Default|SetDMI _returnvalue)
  (bind _returnvalue_2 (Rendering|Material|CreateDynamicMaterialInstance (Variables|Default|GetCenter) 0 0 "None" :!class /Script/Engine.PrimitiveComponent))
  (Variables|Default|SetDMI2 _returnvalue_2)
  (Default|Init (Variables|Default|GetAPC_AudioComponent) "/Game/AdvancedPuzzleConstructor/Sounds/Cue/RotatorStart_Cue.RotatorStart_Cue" 0 0 0.0)
  (Variables|Default|SetCustomState false)
  (Variables|Default|SetCurrPosition (Variables|TelekinesisRotator|GetStartPosition))
  (Variables|Default|SetIsAlreadyCalledAction true))

(event EventButtonPressedBPI
  ;[1 1 1] Button Pressed event. Rotate arrow
  (if (not (Variables|Default|GetInProcess))
    (Variables|Default|SetInProcess true)
    (Default|StarttoLoop (Variables|Default|GetAPC_AudioComponent))
    (Variables|Default|SetStartAngle (* (Variables|Default|GetCurrPosition) -45.0))
    (Variables|Default|SetDestAngle (* (+ (Variables|Default|GetCurrPosition) 1) -45.0))
    (bind _rotcurve (Timeline|Timeline_0 PlayFromStart)
      (:Update
        (Transformation|SetRelativeRotation (Variables|Default|GetCenter) (Math|Rotator|MakeRotator 0.0 (Math|Float|Lerp (Variables|Default|GetStartAngle) (Variables|Default|GetDestAngle) _rotcurve) 0.0) false false))
      (:Finished
        (if (> (+ (Variables|Default|GetCurrPosition) 1) 7)
          (Variables|Default|SetCurrPosition 0)
          (else
            (Variables|Default|SetCurrPosition (+ (Variables|Default|GetCurrPosition) 1))))
        (Variables|Default|SetInProcess false)
        (if (> (Utilities|Array|Length (Variables|TelekinesisRotator|GetTargetActors)) 0)
          ;;[1 1 1] Execute Action
          (if (== (Variables|Default|GetCurrPosition) (Variables|TelekinesisRotator|GetUnlockPosition))
            (for _array_element (Variables|TelekinesisRotator|GetTargetActors)
              (CallFunction|LIBExecuteAction (.Actor (Utilities|Struct|BreakF_ButtonBoxAction _array_element)) (.BoxYep (Utilities|Struct|BreakF_ButtonBoxAction _array_element)))
              (Variables|Default|SetIsAlreadyCalledAction false))
            (elif (not (Variables|Default|GetIsAlreadyCalledAction))
              (for _array_element_2 (Variables|TelekinesisRotator|GetTargetActors)
                (CallFunction|LIBExecuteAction (.Actor (Utilities|Struct|BreakF_ButtonBoxAction _array_element_2)) (.BoxNop (Utilities|Struct|BreakF_ButtonBoxAction _array_element_2)))
                (Variables|Default|SetIsAlreadyCalledAction true))))
          (else
            (CallFunction|LIBDebugPrint (Utilities|String|Append (Utilities|GetDisplayName self) ": TargetActors is empty!") "(R=1.000000,G=0.160801,B=0.000000,A=1.000000)" 3.0)))))))

(event EventSpotObjectBPI
  (params (Spot :type Boolean))
  ;[1 1 1] Spot Object. Turn On / Off light
  (if Spot
    (bind _newtrack_0 (Timeline|Timeline_1 Play)
      (:Update
        (Rendering|Material|SetScalarParameterValue (Variables|Default|GetDMI) "Power" (* _newtrack_0 (Variables|TelekinesisRotator|GetLightPower)) :!class /Script/Engine.MaterialInstanceDynamic)))
    (else
      (Timeline|Timeline_1 Reverse))))

(fn ConstructionScript
  ;[1 1 1] Setup start and unlock positions
  (Transformation|SetRelativeRotation (Variables|Default|GetCenter) (Math|Rotator|MakeRotator 0.0 (* (Variables|TelekinesisRotator|GetStartPosition) -45.0) 0.0) false false)
  (Transformation|SetRelativeRotation (Variables|Default|GetUnlockPos) (Math|Rotator|MakeRotator 0.0 (+ (* (Variables|TelekinesisRotator|GetUnlockPosition) -45.0) 9e+01) 0.0) false false))

(fn GetAngularDampingBPI
  (return 0.0))

(fn GetBoxColorandStateBPI
  (return "NewEnumerator1" false false false))

(fn GetBoxTransformBPI
  (return ""))

(fn GetDeployTimeBPI
  (return 0.0))

(fn GetGrabbingDataBPI
  (return "0, 0, 0" 0.0 0.0 false))

(fn GetObjectAxisBPI
  ;[1 1 1] Return Target Axis. Only Forward vector is required
  (return (Math|Vector|GetForwardVector (Variables|Default|GetArrow)) "0, 0, 0" "0, 0, 0"))

(fn GetObjectTypeBPI
  ;[1 1 1] Return Remote Controlled type
  (return "NewEnumerator5"))

(fn GetPushBoxDataBPI
  (return 0.0 "" ""))

(fn GetTargetTransform
  (return ""))

(fn GetVoltageCapacityBPI
  (return 0.0 0.0))

(fn IsAttachedtoConveyorBPI
  (return false))

(fn IsDeploymentinProgressBPI
  (return false))

(fn IsObjectGrabbedBPI
  (return false))

(fn IsObjectinPickupAreaBPI
  (return false))

(fn IsObjectTeleportableBPI
  (return false))

(fn IsObjectTransportableBPI
  (return false))

(fn IsTelekinesisCompatibleBPI
  ;[1 1 1] Is Telekinesis compatible?
  (return true))

(fn IsTelekinesisPickupableBPI
  (return false))

(fn ObjectCanbeUsed
  ;[1 1 1] Is object can be used?
  (return (not (Variables|Default|GetCustomState))))