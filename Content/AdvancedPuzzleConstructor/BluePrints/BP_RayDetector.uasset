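; Laser ray detector for puzzles that runs configured actions on target actors and plays audio when a player-tagged actor enters its area while enabled.
; The construction script stacks instanced rays by count, spacing and length, then fits the overlap box and audio position to them.
; Activate, Deactivate and FlipFlop events share one timeline that fades the dynamic material's opacity, toggles Enabled on finish and ignores calls while busy.
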(event OnComponentBeginOverlap(OverlapArea)
  (params (OverlappedComponent :type Primitive%20Component%20Object%20Reference) (OtherActor :type Actor%20Object%20Reference) (OtherComp :type Primitive%20Component%20Object%20Reference) (OtherBodyIndex :type Integer) (bFromSweep :type Boolean) (SweepResult :type Hit%20Result%20Structure%20%28by%20ref%29))
  ;[1 1 1] Begin overlap
  (if (Actor|ActorHasTag OtherActor (CallFunction|LIBGetPlayerTag))
    (if (Variables|LaserDetector|GetEnabled)
      (for _array_element (Variables|LaserDetector|GetActors)
        (CallFunction|LIBExecuteAction (.Actor (Utilities|Struct|BreakF_ButtonSimpleAction _array_element)) (.Action (Utilities|Struct|BreakF_ButtonSimpleAction _array_element)))
        (Audio|Components|Audio|Play (Variables|Default|GetAudio) 0.0)))))

(event EventBeginPlay
  ;[1 0.7655 0.1745] Begin Play init
  (Variables|Default|SetIsBusy false)
  (bind _returnvalue (Rendering|Material|CreateDynamicMaterialInstance (Variables|Default|GetDetectorWall) 0 0 "None" :!class /Script/Engine.PrimitiveComponent))
  (bind _output_get (Variables|Default|SetDMI _returnvalue))
  (Rendering|Material|SetVectorParameterValue _output_get "LaserColor" (Variables|LaserDetector|GetColor) :!class /Script/Engine.MaterialInstanceDynamic))

(event EventDeactivateBPI
  ;[1 1 1] Deactivate event
  (if (Variables|LaserDetector|GetEnabled)
    (if (not (Variables|Default|GetIsBusy))
      (Variables|Default|SetIsBusy true)
      ;[1 1 1] Play opacity animation
      (bind _newtrack_0 (Timeline|Timeline_0 PlayFromStart)
        (:Update
          (Rendering|Material|SetScalarParameterValue (Variables|Default|GetDMI) "Opacity" _newtrack_0 :!class /Script/Engine.MaterialInstanceDynamic))
        (:Finished
          (Variables|LaserDetector|SetEnabled (not (Variables|LaserDetector|GetEnabled)))
          (Variables|Default|SetIsBusy false))))))

(event EventActivateBPI
  ;[1 1 1] Activate event
  (if (not (Variables|LaserDetector|GetEnabled))
    (if (not (Variables|Default|GetIsBusy))
      (Variables|Default|SetIsBusy true)
      ;[1 1 1] Play opacity animation
      (bind _newtrack_0 (Timeline|Timeline_0 ReverseFromEnd)
        (:Update
          (Rendering|Material|SetScalarParameterValue (Variables|Default|GetDMI) "Opacity" _newtrack_0 :!class /Script/Engine.MaterialInstanceDynamic))
        (:Finished
          (Variables|LaserDetector|SetEnabled (not (Variables|LaserDetector|GetEnabled)))
          (Variables|Default|SetIsBusy false))))))

(event EventFlipFlopBPI
  ;[1 1 1] Flip Flop event
  (if (Variables|LaserDetector|GetEnabled)
    ;[1 1 1] Deactivate event
    (if (Variables|LaserDetector|GetEnabled)
      (if (not (Variables|Default|GetIsBusy))
        (Variables|Default|SetIsBusy true)
        ;[1 1 1] Play opacity animation
        (bind _newtrack_0 (Timeline|Timeline_0 PlayFromStart)
          (:Update
            (Rendering|Material|SetScalarParameterValue (Variables|Default|GetDMI) "Opacity" _newtrack_0 :!class /Script/Engine.MaterialInstanceDynamic))
          (:Finished
            (Variables|LaserDetector|SetEnabled (not (Variables|LaserDetector|GetEnabled)))
            (Variables|Default|SetIsBusy false)))))
    (else
      ;[1 1 1] Activate event
      (if (not (Variables|LaserDetector|GetEnabled))
        (if (not (Variables|Default|GetIsBusy))
          (Variables|Default|SetIsBusy true)
          (Timeline|Timeline_0 ReverseFromEnd))))))

(fn ConstructionScript
  (bind _raystep (Variables|LaserDetector|GetRayStep))
  (bind _overlapwidth (Variables|LaserDetector|GetOverlapWidth))
  (bind _numrays (Variables|LaserDetector|GetNumRays))
  (bind _lenght (Variables|LaserDetector|GetLenght))
  (bind _overlaparea (Variables|Default|GetOverlapArea))
  (bind _audio (Variables|Default|GetAudio))
  (bind _returnvalue (- _numrays 1))
  (bind _returnvalue_2 (* _returnvalue _raystep))
  (bind _returnvalue_3 (+ _returnvalue_2 _overlapwidth))
  (bind _returnvalue_4 (/ _returnvalue_3 2.0))
  ;[1 1 1] Add ray ISMs and setup location
  (for _index (range 0 (- _numrays 1))
    (Class|InstancedStaticMeshComponent|AddInstanceWorldSpace (Variables|Default|GetDetectorWall) (Math|Transform|MakeTransform (+ (* (Transformation|GetActorUpVector) (* _index (Variables|LaserDetector|GetRayStep))) (Transformation|GetWorldLocation (Variables|Default|GetDetectorWall))) (Transformation|GetActorRotation) (Math|Vector|MakeVector 1.0 (/ _lenght 1e+02) 1.0))))
  (Components|Box|SetBoxExtent _overlaparea (Math|Vector|MakeVector _returnvalue_4 (/ _lenght 2.0) (Variables|LaserDetector|GetOverlapHeight)) true)
  (Transformation|SetRelativeLocation _overlaparea (Math|Vector|MakeVector 0.0 (/ (Variables|LaserDetector|GetLenght) 2.0) (- _returnvalue_4 (/ (Variables|LaserDetector|GetOverlapWidth) 2.0))) false false)
  (Transformation|SetRelativeLocation _audio (+ (Math|Vector|MakeVector 0.0 (/ (Variables|LaserDetector|GetLenght) 2.0) _returnvalue_4) (Variables|/Script/Engine.SceneComponent|GetRelativeLocation _audio)) false false))

(fn IsActorActivatedBPI
  ;[1 1 1] Return default value
  (return false))