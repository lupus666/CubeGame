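; Puzzle conveyor that carries transportable boxes toward a drop point, with reversible direction and optional voltage-based power.
; The construction script builds NumWheels instanced rollers and fits colliders, drop points, indicator and audio to that length.
; Looping timers capture overlapping boxes through interface calls and poll power/activation, while a timeline ramps the speed multiplier for smooth starts and stops.
; Tick spins the rollers, eases captured boxes onto the belt, moves them and releases fallen ones.
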(event Custom|CheckBoxOverlap
  ;[1 1 1] Check if box is overlapping with conveyor
  (bind _array_element (Utilities|Array|ForEachLoopwithBreak (Collision|GetOverlappingActors (Variables|Default|GetOverlapVolume) 0 :!class /Script/Engine.PrimitiveComponent))
    (:LoopBody
      (if (Utilities|DoesObjectImplementInterface _array_element "/Game/AdvancedPuzzleConstructor/BluePrints/Core/BPI_ObjectControls.BPI_ObjectControls_C")
        (bind _transportable (Class|BPIObjectControls|IsObjectTransportableBPI(Message) _array_element))
        (if _transportable
          (bind _attached (Class|BPIObjectControls|IsAttachedtoConveyorBPI(Message) _array_element))
          (if (not _attached)
            (bind _boxtransform (Class|BPIObjectControls|GetBoxTransformBPI(Message) _array_element))
            (Utilities|Array|AddUnique (Variables|Default|GetConveyorCargos) (Utilities|Struct|MakeF_ConveyorData _array_element false 0.0 (CallFunction|GetStartLocation (.location _boxtransform)) (CallFunction|GetDropLocation) (.location _boxtransform)))
            (bind _isattachedtoplayer (Class|BPIObjectControls|GetBoxColorandStateBPI(Message) _array_element))
            (if _isattachedtoplayer
              (Class|BPIObjectControls|DetachfromPlayerBPI(Message) _array_element))
            (Class|BPIObjectControls|SetCustomStateBPI(Message) _array_element true)
            (Class|BPIObjectControls|EnableMeshPhysicBPI(Message) _array_element false)
            (Class|BPIObjectControls|SetAttachedtoConveyorBPI(Message) _array_element true)
            (Class|BPIObjectControls|StartTransitionRotationBPI(Message) _array_element true false)))))))

(event Custom|SetVoltageIndicator
  (params (Voltage :type Float%20%28single-precision%29) (MaxVoltage :type Float%20%28single-precision%29))
  ;[1 1 1] Indicator
  (Class|BPIVoltageIndicator|SetVoltageBPI(Message) (Variables|/Script/Engine.ChildActorComponent|GetChildActor (Variables|Default|GetVoltageIndicator)) Voltage MaxVoltage))

(event Custom|CheckActiveState
  (bind _enabled (Variables|Conveyor|GetEnabled))
  (bind _isactivated (Variables|Default|GetIsActivated))
  ;[1 1 1] State machine. Switch active conveyor state based on voltage and activated / deactivated variable
  (CallFunction|CheckIndicatorVisibility)
  (if (Variables|Conveyor|GetNeedPower)
    (if (> (Variables|Default|GetCurrentVoltage) 0.0)
      (Utilities|FlowControl|Sequence
        (:then_0
          (if (Variables|Conveyor|GetEnabled)
            (Utilities|FlowControl|DoOnce false
              (:Completed
                (CallFunction|ForceActivate :!label _label)))))
        (:then_1
          (if (Variables|Default|GetIsActivated)
            (Utilities|FlowControl|DoOnce false
              (:Completed
                (goto _label)))))
        (:then_2
          (if (Variables|Conveyor|GetEnabled)
            (if (not (Variables|Default|GetIsActivated))
              (CallFunction|ForceDeactivate)))))
      (elif (Variables|Conveyor|GetEnabled)
        (CallFunction|ForceDeactivate)
        (CallFunction|ResetPowerStart)
        (CallFunction|ResetWantStart)))
    (else
      (Utilities|FlowControl|Sequence
        (:then_0
          (if _isactivated
            (if (not _enabled)
              (CallFunction|ForceActivate))))
        (:then_1
          (if (not _isactivated)
            (if _enabled
              (CallFunction|ForceDeactivate))))))))

(event Custom|ForceDeactivate
  ;[1 1 1] Force activate / deactivate state. Execute smooth start / stop for conveyor rotation
  (CallFunction|ManageSound false)
  (Variables|Conveyor|SetEnabled false)
  (Variables|Default|SetUpdateRotation false)
  (CallFunction|ResetSmoothActivate)
  (Utilities|FlowControl|DoOnce false
    (:Completed
      (bind _newtrack_0 (Timeline|StopRotation ReverseFromEnd)
        (:Update
          (Variables|Default|SetTickMultiplier _newtrack_0))))))

(event Custom|ResetWantStart
  ;[1 1 1] State machine. Switch active conveyor state based on voltage and activated / deactivated variable
  (Utilities|FlowControl|DoOnce false) ; enters at Reset
)

(event Custom|BlinkRedNormal
  (bind _instancedstaticmesh (Variables|Default|GetInstancedStaticMesh))
  (bind _blinkmaterial (Variables|Default|GetBlinkMaterial))
  ;[1 1 1] Blink lamps when switch conveyr direction
  (Rendering|Material|SetVectorParameterValue _blinkmaterial "Color" "(R=0.505208,G=0.013780,B=0.000000,A=1.000000)" :!class /Script/Engine.MaterialInstanceDynamic)
  (Rendering|SetRenderCustomDepth _instancedstaticmesh true)
  (Utilities|FlowControl|Delay (Variables|Conveyor|GetBlinkTime))
  (Rendering|Material|SetVectorParameterValue _blinkmaterial "Color" "(R=0.489583,G=0.938756,B=1.000000,A=1.000000)" :!class /Script/Engine.MaterialInstanceDynamic)
  (Rendering|SetRenderCustomDepth _instancedstaticmesh false))

(event Custom|ManageSound
  (params (StartSound :type Boolean))
  (bind _apc_audiocomponent (Variables|Default|GetAPC_AudioComponent))
  ;[1 1 1] Sound manager
  (if StartSound
    (Default|StarttoLoop _apc_audiocomponent)
    (else
      (Default|StopAll _apc_audiocomponent))))

(event Custom|CheckIndicatorVisibility
  ;[1 1 1] Show voltage indicator if requred Power Box
  (if (Variables|Conveyor|GetNeedPower)
    (if (> (Variables|Default|GetCurrentVoltage) 0.0)
      (CallFunction|ShowHideIndicator false :!label _label)
      (else
        (CallFunction|ShowHideIndicator true)))
    (else
      (goto _label))))

(event Custom|ResetSmoothDeactivate
  ;[1 1 1] Force activate / deactivate state. Execute smooth start / stop for conveyor rotation
  (Utilities|FlowControl|DoOnce false) ; enters at Reset
)

(event Custom|ResetSmoothActivate
  ;[1 1 1] Force activate / deactivate state. Execute smooth start / stop for conveyor rotation
  (Utilities|FlowControl|DoOnce false) ; enters at Reset
)

(event Custom|ShowHideIndicator
  (params (Show :type Boolean))
  ;[1 1 1] Indicator
  (Class|BPIVoltageIndicator|HideIndicatorBPI(Message) (Variables|/Script/Engine.ChildActorComponent|GetChildActor (Variables|Default|GetVoltageIndicator)) Show))

(event Custom|ResetPowerStart
  ;[1 1 1] State machine. Switch active conveyor state based on voltage and activated / deactivated variable
  (Utilities|FlowControl|DoOnce false) ; enters at Reset
)

(event Custom|StopRotationConv
  ;[1 1 1] Force activate / deactivate state. Execute smooth start / stop for conveyor rotation
  (bind _newtrack_0 (Timeline|StopRotation ReverseFromEnd)
    (:Update
      (Variables|Default|SetTickMultiplier _newtrack_0))))

(event Custom|StartRotationConv
  ;[1 1 1] Force activate / deactivate state. Execute smooth start / stop for conveyor rotation
  (bind _newtrack_0 (Timeline|StopRotation PlayFromStart)
    (:Update
      (Variables|Default|SetTickMultiplier _newtrack_0))))

(event Custom|ForceActivate
  ;[1 1 1] Force activate / deactivate state. Execute smooth start / stop for conveyor rotation
  (if (Variables|Default|GetUpdateRotation)
    _
    (else
      (CallFunction|ManageSound true)
      (Variables|Conveyor|SetEnabled true)
      (Variables|Default|SetUpdateRotation true)))
  (CallFunction|ResetSmoothDeactivate)
  (Utilities|FlowControl|DoOnce false
    (:Completed
      (bind _newtrack_0 (Timeline|StopRotation PlayFromStart)
        (:Update
          (Variables|Default|SetTickMultiplier _newtrack_0))))))

(event EventBeginPlay
  ;[1 0.7655 0.1745] Begin Play init
  (Default|Init (Variables|Default|GetAPC_AudioComponent) 0 0 "/Game/AdvancedPuzzleConstructor/Sounds/Cue/Conveyor_Cue.Conveyor_Cue" 1.0)
  (Variables|Default|SetUpdateRotation false)
  (CallFunction|ShowHideIndicator (Variables|Conveyor|GetNeedPower))
  (CallFunction|SetVoltageIndicator 0.0 0.0)
  (Variables|Default|SetCurrentVoltage 0.0)
  (Variables|Default|SetRotationAngle 0.0)
  (Utilities|Array|Clear (Variables|Default|GetConveyorCargos))
  (bind _returnvalue (Utilities|Time|SetTimerbyFunctionName 0 "CheckBoxOverlap" 0.1 true))
  (bind _output_get (Variables|Default|SetCheckIsBoxPlacedTimeHandle _returnvalue))
  (Utilities|Time|UnpauseTimerbyHandle _output_get)
  (bind _returnvalue_2 (Utilities|Time|SetTimerbyFunctionName 0 "CheckActiveState" 0.2 true))
  (bind _output_get_2 (Variables|Default|SetCheckActivationTimeHanlde _returnvalue_2))
  (Utilities|Time|UnpauseTimerbyHandle _output_get_2)
  (bind _returnvalue_3 (Rendering|Material|CreateDynamicMaterialInstance (Variables|Default|GetInstancedStaticMesh) 1 0 "None" :!class /Script/Engine.PrimitiveComponent))
  (Variables|Default|SetBlinkMaterial _returnvalue_3)
  (if (Variables|Conveyor|GetEnabled)
    (CallFunction|ActivateBPI)
    (if (not (Variables|Conveyor|GetNeedPower))
      (CallFunction|ForceActivate))))

(event EventTick
  (params (DeltaSeconds :type Float%20%28single-precision%29))
  (bind _returnvalue (Transformation|GetActorRotation))
  (bind _speed (Variables|Conveyor|GetSpeed))
  (bind _instancedstaticmesh (Variables|Default|GetInstancedStaticMesh))
  (bind (_roll _pitch _yaw) (Math|Rotator|BreakRotator _returnvalue))
  (bind _returnvalue_2 (* _speed 1.25))
  (bind _output_get (Variables|Default|SetDeltaTime DeltaSeconds))
  ;[1 1 1] Update rotation for all ISMs
  (CallFunction|UpdateCargoLocationandTransition _output_get (Variables|Default|GetTickMultiplier) (Variables|Conveyor|GetSpeed) (Variables|Conveyor|GetTransitionSpeed))
  (Variables|Default|SetRotationAngle (+ (Variables|Default|GetRotationAngle) (* (Variables|Default|GetTickMultiplier) (Math|Float|SelectFloat (* _returnvalue_2 -1.0) _returnvalue_2 (Utilities|Enum|Equal(Enum) (Variables|Conveyor|GetDirection) "NewEnumerator0")))))
  (for _index (range 0 (- (Variables|Conveyor|GetNumWheels) 2))
    (Components|InstancedStaticMesh|UpdateInstanceTransform _instancedstaticmesh _index (Math|Transform|MakeTransform (+ (* (Math|Vector|GetForwardVector (Variables|Default|GetArrow)) (* _index (Variables|Default|GetInstanceStep))) (Transformation|GetWorldLocation _instancedstaticmesh)) (Math|Rotator|MakeRotator (Variables|Default|GetRotationAngle) _pitch _yaw)) true false false))
  (Components|InstancedStaticMesh|UpdateInstanceTransform _instancedstaticmesh (- (Variables|Conveyor|GetNumWheels) 1) (Math|Transform|MakeTransform (+ (* (Math|Vector|GetForwardVector (Variables|Default|GetArrow)) (* _index (Variables|Default|GetInstanceStep))) (Transformation|GetWorldLocation _instancedstaticmesh)) (Math|Rotator|MakeRotator (Variables|Default|GetRotationAngle) _pitch _yaw)) true true false))

(event EventActivateBPI
  ;[1 1 1] Activate / Deactivate events
  (Variables|Default|SetIsActivated true)
  (CallFunction|ResetWantStart))

(event EventDeactivateBPI
  ;[1 1 1] Activate / Deactivate events
  (Variables|Default|SetIsActivated false))

(event EventChangeConveyorDirectionBPI
  (bind _conveyorcargos (Variables|Default|GetConveyorCargos))
  ;[1 1 1] Change conveyor direction event
  (if (Variables|Conveyor|GetNeedPower)
    (if (> (Variables|Default|GetCurrentVoltage) 5.0)
      (if (Variables|Default|GetUpdateRotation) :!label _label
        (CallFunction|BlinkRedNormal)
        (CallFunction|StopRotationConv)
        (Utilities|FlowControl|Delay (Components|Timeline|GetTimelineLength (Variables|Default|GetStopRotation)))
        (if (Utilities|Enum|Equal(Enum) (Variables|Conveyor|GetDirection) "NewEnumerator0")
          (Variables|Conveyor|SetDirection "NewEnumerator1")
          (else
            (Variables|Conveyor|SetDirection "NewEnumerator0")))
        (for (_array_element _array_index) _conveyorcargos
          (Utilities|Array|SetArrayElem _conveyorcargos _array_index (Utilities|Struct|MakeF_ConveyorData (.actor _array_element) (.readytoconveyor _array_element) (.transitioncounter _array_element) (.startconveyorlocation _array_element) (CallFunction|GetDropLocation) (.starttransitionlocation _array_element))))
        (CallFunction|StartRotationConv)))
    (else
      (goto _label))))

(event EventConnectPowerBPI
  (params (Voltage :type Float%20%28single-precision%29) (MaxVoltage :type Float%20%28single-precision%29) (DischargeSpeed :type Float%20%28single-precision%29))
  ;[1 1 1] Power connect, disconnect, reconnect
  (bind _output_get (Variables|Default|SetCurrentVoltage Voltage))
  (CallFunction|SetVoltageIndicator _output_get MaxVoltage))

(event EventDisconnectPowerBPI
  ;[1 1 1] Power connect, disconnect, reconnect
  (Variables|Default|SetCurrentVoltage 0.0))

(event EventReconnectPowerBPI
  ;[1 1 1] Power connect, disconnect, reconnect
  (CallFunction|ResetWantStart))

(fn ConstructionScript
  (bind _apc_audiocomponent (Variables|Default|GetAPC_AudioComponent))
  (bind _instancestep (Variables|Default|GetInstanceStep))
  (bind _numwheels (Variables|Conveyor|GetNumWheels))
  (bind _arrow (Variables|Default|GetArrow))
  (bind _overlapvolume (Variables|Default|GetOverlapVolume))
  (bind _voltageindicator (Variables|Default|GetVoltageIndicator))
  (bind _maincollider (Variables|Default|GetMainCollider))
  (bind _instancedstaticmesh (Variables|Default|GetInstancedStaticMesh))
  (bind _instancedstaticmesh_2 (Variables|Default|GetInstancedStaticMesh))
  (bind _arrow_2 (Variables|Default|GetArrow))
  (bind _arrow_3 (Variables|Default|GetArrow))
  (bind _instancestep_2 (Variables|Default|GetInstanceStep))
  (bind _numwheels_2 (Variables|Conveyor|GetNumWheels))
  (bind _returnvalue (- _numwheels_2 1))
  (bind _returnvalue_2 (- _numwheels 1))
  (bind _returnvalue_3 (Transformation|GetWorldLocation _instancedstaticmesh_2))
  (bind _returnvalue_4 (Math|Vector|GetForwardVector _arrow))
  (bind _returnvalue_5 (Math|Vector|GetForwardVector _arrow_3))
  (bind _returnvalue_6 (Math|Vector|GetForwardVector _arrow_2))
  (bind _returnvalue_7 (Transformation|GetWorldLocation _instancedstaticmesh))
  (bind _boxextent (Variables|/Script/Engine.BoxComponent|GetBoxExtent _overlapvolume))
  (bind _boxextent_2 (Variables|/Script/Engine.BoxComponent|GetBoxExtent _maincollider))
  (bind _returnvalue_8 (* _returnvalue _instancestep_2))
  (bind _returnvalue_9 (* _returnvalue_2 _instancestep))
  (bind (_x _y _z) (Math|Vector|BreakVector _boxextent))
  (bind (_x_2 _y_2 _z_2) (Math|Vector|BreakVector _boxextent_2))
  (bind _returnvalue_10 (/ _returnvalue_8 2.0))
  (bind _returnvalue_11 (/ _returnvalue_9 2.0))
  (bind _returnvalue_12 (* _returnvalue_5 _returnvalue_10))
  (bind _returnvalue_13 (* _returnvalue_4 _returnvalue_11))
  (bind _returnvalue_14 (+ _returnvalue_7 _returnvalue_12))
  (bind (_x_3 _y_3) (Math|Vector|BreakVector _returnvalue_14))
  ;[1 1 1] Setup location for ISMs, Drop points, voltage indicator, APC audio
  (for _index (range 0 (- (Variables|Conveyor|GetNumWheels) 1))
    (Class|InstancedStaticMeshComponent|AddInstanceWorldSpace (Variables|Default|GetInstancedStaticMesh) (Math|Transform|MakeTransform (+ (* (Transformation|GetActorRightVector) (* _index (Variables|Default|GetInstanceStep))) (Transformation|GetWorldLocation (Variables|Default|GetInstancedStaticMesh))) (Transformation|GetActorRotation))))
  (Transformation|SetWorldLocation (Variables|Default|GetRightDropPoint) (+ (+ _returnvalue_3 (* _returnvalue_6 (+ (* (- (Variables|Conveyor|GetNumWheels) 1) (Variables|Default|GetInstanceStep)) (Variables|Conveyor|GetDropPointOffset)))) "0, 0,100.000000") false false)
  (Transformation|SetWorldLocation (Variables|Default|GetLeftDropPoint) (+ (+ _returnvalue_3 (* (* _returnvalue_6 -1.0) (Variables|Conveyor|GetDropPointOffset))) "0, 0,100.000000") false false)
  (Transformation|SetWorldLocation _voltageindicator (+ (Transformation|GetWorldLocation _voltageindicator) _returnvalue_13) false false)
  (Transformation|SetWorldLocation _apc_audiocomponent (+ (Transformation|GetWorldLocation _apc_audiocomponent) _returnvalue_13) false false)
  (Transformation|SetWorldLocation _overlapvolume (Math|Vector|MakeVector _x_3 _y_3 (.Z (Math|Vector|BreakVector (Transformation|GetWorldLocation _overlapvolume)))) false false)
  (Components|Box|SetBoxExtent _overlapvolume (Math|Vector|MakeVector _x _returnvalue_10 _z) true)
  (Transformation|SetWorldLocation _maincollider (Math|Vector|MakeVector _x_3 _y_3 (.Z (Math|Vector|BreakVector (Transformation|GetWorldLocation _maincollider)))) false false)
  (Components|Box|SetBoxExtent _maincollider (Math|Vector|MakeVector _x_2 (+ _returnvalue_10 (/ (Variables|Default|GetInstanceStep) 2.0)) _z_2) true))

(fn GetDropLocation
  ;[1 1 1] Get Box drop down location based on conveyor rotation direction
  (return (Math|Vector|SelectVector (Transformation|GetWorldLocation (Variables|Default|GetLeftDropPoint)) (Transformation|GetWorldLocation (Variables|Default|GetRightDropPoint)) (Utilities|Enum|Equal(Enum) (Variables|Conveyor|GetDirection) "NewEnumerator0"))))

(fn GetStartLocation
  (params (MeshLocation :type Vector))
  (bind _returnvalue (Transformation|GetActorLocation))
  (bind (_x _y) (Math|Vector|BreakVector MeshLocation))
  (bind (_x_2 _y_2) (Math|Vector|BreakVector _returnvalue))
  ;[1 1 1] Get start conveyor location
  (return (+ (* (Transformation|GetActorRightVector) (Math|Vector|VectorLength (- (Math|Vector|MakeVector _x_2 _y_2 0.0) (Math|Vector|MakeVector _x _y 0.0)))) _returnvalue "0,0,124.000000")))

(fn UpdateCargoLocationandTransition
  (params (Time :type Float%20%28single-precision%29) (Multiplier :type Float%20%28single-precision%29) (Speed :type Float%20%28single-precision%29) (TransitSpeed :type Float%20%28single-precision%29))
  (bind _conveyorcargos (Variables|Default|GetConveyorCargos))
  ;[1 1 1] Move all Boxes by the conveyor direction. Check if is any Box is falling down
  (LocalVariables|SetFrameTime Time)
  (LocalVariables|SetMult Multiplier)
  (LocalVariables|SetInSpeed Speed)
  (LocalVariables|SetTrSpeed TransitSpeed)
  (if (> (Utilities|Array|Length _conveyorcargos) 0)
    (for (_array_element _array_index) _conveyorcargos
      (LocalVariables|SetActor (.Actor (Utilities|Struct|BreakF_ConveyorData _array_element)))
      (LocalVariables|SetReady (.ReadyToConveyor (Utilities|Struct|BreakF_ConveyorData _array_element)))
      (LocalVariables|SetTransCounter (.TransitionCounter (Utilities|Struct|BreakF_ConveyorData _array_element)))
      (LocalVariables|SetStartLoc (.StartConveyorLocation (Utilities|Struct|BreakF_ConveyorData _array_element)))
      (LocalVariables|SetEndLoc (.EndConveyorLocation (Utilities|Struct|BreakF_ConveyorData _array_element)))
      (LocalVariables|SetStartTransLoc (.StartTransitionLocation (Utilities|Struct|BreakF_ConveyorData _array_element)))
      (if (LocalVariables|GetReady)
        (LocalVariables|SetConvCounter (Math|Float|Clamp(Float) (+ (* (* (LocalVariables|GetInSpeed) 0.1) (* (LocalVariables|GetFrameTime) (LocalVariables|GetMult))) (LocalVariables|GetConvCounter))))
        (bind _boxtransform (Class|BPIObjectControls|GetBoxTransformBPI(Message) (LocalVariables|GetActor)))
        (Class|BPIObjectControls|SetBoxLocationBPI(Message) (LocalVariables|GetActor) (Math|Vector|MakeVector (.x (+ (Math|Vector|MakeVector (.X (Math|Vector|BreakVector (.location _boxtransform))) (.Y (Math|Vector|BreakVector (.location _boxtransform))) 0.0) (* (Math|Vector|Normalize (- (Math|Vector|MakeVector (.x (LocalVariables|GetEndLoc)) (.y (LocalVariables|GetEndLoc)) 0.0) (Math|Vector|MakeVector (.X (Math|Vector|BreakVector (.location _boxtransform))) (.Y (Math|Vector|BreakVector (.location _boxtransform))) 0.0))) (* (LocalVariables|GetInSpeed) (* (LocalVariables|GetMult) (LocalVariables|GetFrameTime)) 6e+01)))) (.y (+ (Math|Vector|MakeVector (.X (Math|Vector|BreakVector (.location _boxtransform))) (.Y (Math|Vector|BreakVector (.location _boxtransform))) 0.0) (* (Math|Vector|Normalize (- (Math|Vector|MakeVector (.x (LocalVariables|GetEndLoc)) (.y (LocalVariables|GetEndLoc)) 0.0) (Math|Vector|MakeVector (.X (Math|Vector|BreakVector (.location _boxtransform))) (.Y (Math|Vector|BreakVector (.location _boxtransform))) 0.0))) (* (LocalVariables|GetInSpeed) (* (LocalVariables|GetMult) (LocalVariables|GetFrameTime)) 6e+01)))) (.Z (Math|Vector|BreakVector (.location _boxtransform)))))
        (if (< (- (.Z (Math|Vector|BreakVector (.location _boxtransform))) (.z (LocalVariables|GetEndLoc))) 1e+01)
          (Class|BPIObjectControls|SetAttachedtoConveyorBPI(Message) (LocalVariables|GetActor) false)
          (Class|BPIObjectControls|SetCustomStateBPI(Message) (LocalVariables|GetActor) false)
          (Utilities|Array|RemoveIndex _conveyorcargos _array_index)
          (else
            (Utilities|Array|SetArrayElem _conveyorcargos _array_index (Utilities|Struct|MakeF_ConveyorData (LocalVariables|GetActor) (LocalVariables|GetReady) (LocalVariables|GetTransCounter) (LocalVariables|GetStartLoc) (LocalVariables|GetEndLoc) (LocalVariables|GetStartTransLoc)) :!label _label)))
        (else
          (bind _output_get (LocalVariables|SetTransCounter (Math|Float|Clamp(Float) (+ (LocalVariables|GetTransCounter) (* (LocalVariables|GetFrameTime) (LocalVariables|GetTrSpeed))))))
          (LocalVariables|SetReady (>= _output_get 1.0))
          (Class|BPIObjectControls|SetBoxLocationBPI(Message) (LocalVariables|GetActor) (Math|Interpolation|Ease "EaseInOut" (Math|Float|Clamp(Float) (+ (LocalVariables|GetTransCounter) (* (LocalVariables|GetFrameTime) (LocalVariables|GetTrSpeed)))) (LocalVariables|GetStartTransLoc) (LocalVariables|GetStartLoc) 2.0))
          (Class|BPIObjectControls|EnableMeshPhysicBPI(Message) (LocalVariables|GetActor) true)
          (goto _label))))))

(fn IsActorActivatedBPI
  ;[1 1 1] Return actor state
  (return (Variables|Conveyor|GetEnabled)))